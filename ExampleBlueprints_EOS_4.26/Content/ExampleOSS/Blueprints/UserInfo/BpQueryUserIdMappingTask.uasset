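; Task actor that looks up an online user ID from a display name or email through the Online Subsystem user interface.
; It runs an async user ID mapping query as the first local player's net ID.
; It reports the found ID, or a failure message with any error, through CallOnComplete, then destroys itself.
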(event `self.Query User Id Mapping`
  (params (`Display Name Input` :type String))
  (bind (_bwassuccessful _userid _displaynameoremail _founduserid _error) (`OnlineUserSubsystemQueryUserIdMapping.QueryUserIdMapping` (subsystem `OnlineUserSubsystem`) (`OnlineHelpers.GetControllerUniqueNetId` (`GameplayStatics.GetPlayerController` 0)) `Display Name Input`)
    (:`OnCallFailed`
      (`self.On Complete` "Unable to lookup user by display name."))
    (:`OnQueryUserMappingComplete`
      (if _bwassuccessful
        (`self.On Complete` (`KismetStringLibrary.Concat_StrStr` "Found: " (`OnlineHelpers.Conv_FUniqueNetIdReplToString` _founduserid)))
        (else
          (`self.On Complete` (`KismetStringLibrary.Concat_StrStr` "Unable to lookup user by display name: " _error))))))
  (`self.K2_DestroyActor`))

(fn `UserConstructionScript`
  (`parent.UserConstructionScript`))