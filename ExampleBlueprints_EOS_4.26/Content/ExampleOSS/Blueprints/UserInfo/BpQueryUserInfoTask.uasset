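; Short-lived task actor in the OSS example that looks up a user's display name from an EOS Product User ID and Epic account ID.
; It joins both IDs with "|" into a unique player ID, then runs an async user info query through the Online User subsystem.
; On success it reads the cached user info; either way it reports a message through CallOnComplete and destroys itself.
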(event `self.Query User Info`
  (params (PUID :type String) (`Epic ID` :type String))
  ;[0 0 0] This behaviour is specific to EOS, and we form the actual user ID based on the inputs.
  (bind _returnvalue (`OnlineIdentitySubsystem.CreateUniquePlayerId` (subsystem `OnlineIdentitySubsystem`) (`KismetStringLibrary.Concat_StrStr` PUID "|" `Epic ID`)))
  ;[0 0 0] Lookup the user information and cache it.
  (bind (_bwassuccessful _userids _errorstr) (`OnlineUserSubsystemQueryUserInfo.QueryUserInfo` (subsystem `OnlineUserSubsystem`) 0 (`|MakeArray` _returnvalue))
    (:`OnCallFailed`
      (`self.On Complete` "Unable to lookup user info.")
      (`self.K2_DestroyActor` :!label _label))
    (:`OnQueryUserInfoComplete`
      (if _bwassuccessful
        ;[0 0 0] Retrieve the actual user information from the cache and return the user's display name.
        (bind _returnvalue_2 (`OnlineUserSubsystem.GetUserInfo` (subsystem `OnlineUserSubsystem`) 0 _returnvalue))
        (`self.On Complete` (`KismetStringLibrary.Concat_StrStr` "Found user: " (`OnlineUserRef.GetDisplayName` _returnvalue_2)))
        (`self.K2_DestroyActor`)
        (else
          (`self.On Complete` (`KismetStringLibrary.Concat_StrStr` "Unable to lookup user info: " _errorstr))
          (goto _label))))))

(fn `UserConstructionScript`
  (`parent.UserConstructionScript`))