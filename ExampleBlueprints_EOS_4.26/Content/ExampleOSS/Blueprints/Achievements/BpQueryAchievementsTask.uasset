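; Task actor that fetches the first local player's achievements from the online achievements subsystem and reports them through an OnComplete callback.
; It queries achievement descriptions, then achievement progress, then merges both cached sets into achievement data entries.
; An entry counts as unlocked at 100 progress, which also selects the unlocked or locked description text.
; Any failure returns an unsuccessful empty result, and the actor destroys itself after either outcome.
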(event `self.Query Achievements`
  (bind (_localuserid _bwassuccessful) (`OnlineAchievementsSubsystemQueryAchievementDescriptions.QueryAchievementDescriptions` (subsystem `OnlineAchievementsSubsystem`) (`OnlineHelpers.GetControllerUniqueNetId` (`GameplayStatics.GetPlayerController` 0)))
    (:`OnCallFailed`
      (`self.On Complete` false (`|MakeArray`) :!label _label)
      (`self.K2_DestroyActor`))
    (:`OnQueryAchievementsComplete`
      (if _bwassuccessful
        (bind (_localuserid_2 _bwassuccessful_2) (`OnlineAchievementsSubsystemQueryAchievements.QueryAchievements` (subsystem `OnlineAchievementsSubsystem`) (`OnlineHelpers.GetControllerUniqueNetId` (`GameplayStatics.GetPlayerController` 0)))
          (:`OnCallFailed`
            (goto _label))
          (:`OnQueryAchievementsComplete`
            (if _bwassuccessful_2
              (bind (_outachievements _returnvalue) (`OnlineAchievementsSubsystem.GetCachedAchievements` (subsystem `OnlineAchievementsSubsystem`) (`OnlineHelpers.GetControllerUniqueNetId` (`GameplayStatics.GetPlayerController` 0))))
              (if (`|EnumEquality` _returnvalue "Success")
                (set `self.Results` (`|MakeArray`))
                (for _array_element _outachievements
                  (bind (_id _progress) (break `OnlineAchievementBP` _array_element))
                  (bind _outachievementdesc (`OnlineAchievementsSubsystem.GetCachedAchievementDescription` (subsystem `OnlineAchievementsSubsystem`) _id))
                  (bind _returnvalue_2 (`KismetMathLibrary.NearlyEqual_FloatFloat` _progress 100.0))
                  (`KismetArrayLibrary.Array_Add` (`self.Results`) (make `/Game/ExampleOSS/Common/BaseTasks/Achievements/AchievementData` _id (break `OnlineAchievementDescBP` _outachievementdesc) (select `bool` _returnvalue_2 :`false` (`.LockedDesc` (break `OnlineAchievementDescBP` _outachievementdesc)) :`true` (`.UnlockedDesc` (break `OnlineAchievementDescBP` _outachievementdesc))) _returnvalue_2 _progress)))
                (`self.On Complete` true (`self.Results`))
                (`self.K2_DestroyActor`)
                (else
                  (goto _label)))
              (else
                (goto _label)))))
        (else
          (goto _label))))))

(fn `UserConstructionScript`
  (`parent.UserConstructionScript`))