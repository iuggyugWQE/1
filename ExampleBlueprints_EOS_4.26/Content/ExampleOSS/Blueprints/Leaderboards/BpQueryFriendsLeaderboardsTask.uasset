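; Task actor that queries friends' leaderboard scores through the online subsystem and reports the results.
; QueryFriendsLeaderboards builds a read object for the TestScore integer column and calls ReadLeaderboardsForFriends for local user 0.
; Returned rows become entry structs, with score taken from the queried column as EOS places it there for friend searches.
; It fires OnComplete with success or an empty failure, then destroys itself.
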(event `self.Query Friends Leaderboards`
  (bind _array (`|MakeArray`))
  (bind _returnvalue (`|GenericCreateObject` "/Script/OnlineSubsystemBlueprints.OnlineLeaderboardRead" self))
  (`OnlineLeaderboardRead.SetColumns` _returnvalue (`|MakeArray` (make `ColumnMetaDataBP` "TestScore" "Int32")))
  (bind _bwassuccessful (`OnlineLeaderboardsSubsystemReadLeaderboardsForFriends.ReadLeaderboardsForFriends` (subsystem `OnlineLeaderboardsSubsystem`) 0 _returnvalue)
    (:`OnCallFailed`
      (`self.On Complete` false _array :!label _label)
      (`self.K2_DestroyActor`))
    (:`OnLeaderboardReadComplete`
      (if _bwassuccessful
        (set `self.Results` _array)
        (for _array_element (`OnlineLeaderboardRead.GetRows` _returnvalue)
          (`KismetArrayLibrary.Array_Add` (`self.Results`) (make `/Game/ExampleOSS/Common/BaseTasks/Leaderboards/LeaderboardEntryData` (`.Rank` (break `OnlineStatsRowBP` _array_element)) (`OnlineHelpers.Conv_FUniqueNetIdReplToString` (`.PlayerId` (break `OnlineStatsRowBP` _array_element))) (break `OnlineStatsRowBP` _array_element) (`.AsInt` (break `VariantDataBP` (`BlueprintMapLibrary.Map_Find` (`.Columns` (break `OnlineStatsRowBP` _array_element)) "TestScore"))))))
        (`self.On Complete` true (`self.Results`))
        (`self.K2_DestroyActor`)
        (else
          (goto _label))))))

(fn `UserConstructionScript`
  (`parent.UserConstructionScript`))