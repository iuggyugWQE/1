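; One-shot task actor that queries the local player's "TestLatest" and "TestScore" stats from the online subsystem in the ExampleOSS example.
; QueryStats runs an async stats query using the first player controller's unique net ID.
; On success, it converts the first user's stats into name and integer pairs and passes them to CallOnComplete.
; Failure reports an empty result, and the actor destroys itself on either outcome.
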(event `self.Query Stats`
  (bind _array (`|MakeArray`))
  (bind _returnvalue (`OnlineHelpers.GetControllerUniqueNetId` (`GameplayStatics.GetPlayerController` 0)))
  (bind (_resultstate _usersstatsresult) (`OnlineStatsSubsystemQueryStats.QueryStats` (subsystem `OnlineStatsSubsystem`) _returnvalue (`|MakeArray` _returnvalue) (`|MakeArray` "TestLatest" "TestScore"))
    (:`OnCallFailed`
      (`self.On Complete` false _array :!label _label)
      (`self.K2_DestroyActor`))
    (:`OnlineStatsQueryUsersStatsComplete`
      (if (`.Successful` (break `OnlineErrorInfo` _resultstate))
        (set `self.Results` _array)
        (bind (_playerid _stats) (break `OnlineStatsUserStatsBP` (`|GetArrayItem` _usersstatsresult)))
        (bind _keys (`BlueprintMapLibrary.Map_Keys` _stats))
        (for _array_element _keys
          (`KismetArrayLibrary.Array_Add` (`self.Results`) (make `/Game/ExampleOSS/Common/BaseTasks/Stats/StatData` _array_element (`.AsInt` (break `VariantDataBP` (`BlueprintMapLibrary.Map_Find` _stats _array_element))))))
        (`self.On Complete` true (`self.Results`))
        (`self.K2_DestroyActor`)
        (else
          (goto _label))))))

(fn `UserConstructionScript`
  (`parent.UserConstructionScript`))