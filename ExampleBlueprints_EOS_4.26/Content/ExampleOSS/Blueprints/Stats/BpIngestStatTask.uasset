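; Short-lived task actor that writes a single named stat for the local player through the online stats subsystem.
; IngestStat sends an Int32 Set update for the first player controller's user id via the async UpdateStats call.
; Success or failure is reported through CallOnComplete, after which the actor destroys itself.
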(event `self.Ingest Stat`
  (params (`Stat Name` :type String) (`Ingest Amount` :type Integer))
  (bind _returnvalue (`OnlineHelpers.GetControllerUniqueNetId` (`GameplayStatics.GetPlayerController` 0)))
  (bind _resultstate (`OnlineStatsSubsystemUpdateStats.UpdateStats` (subsystem `OnlineStatsSubsystem`) _returnvalue (`|MakeArray` (make `OnlineStatsUserUpdatedStatsBP` _returnvalue (`|MakeMap` `Stat Name` (make `OnlineStatUpdateBP` "Set" (make `VariantDataBP` "Int32" false `Ingest Amount`))))))
    (:`OnCallFailed`
      (`self.On Complete` false))
    (:`OnlineStatsUpdateStatsComplete`
      (`self.On Complete` (`.Successful` (break `OnlineErrorInfo` _resultstate)))))
  (`self.K2_DestroyActor`))

(fn `UserConstructionScript`
  (`parent.UserConstructionScript`))