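; Multiplayer task in an Online Subsystem example that registers each connecting player with the local named session.
; On player connect, it reads the controller's unique net ID and caches it on MultiplayerPlayerState, because the controller no longer has it at logout when unregistering needs it.
; It then calls the async RegisterPlayers with that ID and prints an error if the call or registration fails.
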(event `self.On Player Connected`
  (params (`Player Controller` :type "PlayerController Object Reference"))
  ;[0 0 0] When a player disconnects, their unique net ID has already been removed from their PlayerController, so we won't be able to use "Get Controller Unique Net Id" during OnLogout. Store it separately in the player state here so we can use that to unregister the player properly.
  (bind _output_get (set `/Game/ExampleOSS/Common/Multiplayer/MultiplayerPlayerState.Unique Net Id` (`OnlineHelpers.GetControllerUniqueNetId` `Player Controller`) (cast `/Game/ExampleOSS/Common/Multiplayer/MultiplayerPlayerState` (`Controller.PlayerState` `Player Controller`) :!pure true)))
  (bind (_sessionname _playerids _bwassuccessful) (`OnlineSessionSubsystemRegisterPlayers.RegisterPlayers` (subsystem `OnlineSessionSubsystem`) "MyLocalSessionName" (`|MakeArray` _output_get))
    (:`OnCallFailed`
      (`KismetSystemLibrary.PrintString` "Failed to register player." :!label _label))
    (:`OnRegisterPlayersComplete`
      (if (not _bwassuccessful)
        (goto _label)))))

(fn `UserConstructionScript`
  (`parent.UserConstructionScript`))