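; Example Blueprint from ExampleOSS that reports which online subsystem services are available.
; Each function fetches one Online subsystem, covering identity, friends, sessions, lobbies, parties, presence, achievements, leaderboards, stats, user info and cloud or title files, and returns its IsSubsystemAvailable result.
; It holds no state or events, only these independent availability queries.
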(fn `Achievements Available?`
  (returns (Available :type Boolean))
  (return (`OnlineAchievementsSubsystem.IsSubsystemAvailable` (subsystem `OnlineAchievementsSubsystem`))))

(fn `Auth Available?`
  (returns (Available :type Boolean))
  (return (`OnlineIdentitySubsystem.IsSubsystemAvailable` (subsystem `OnlineIdentitySubsystem`))))

(fn `Friends Available?`
  (returns (Available :type Boolean))
  (return (`OnlineFriendsSubsystem.IsSubsystemAvailable` (subsystem `OnlineFriendsSubsystem`))))

(fn `Leaderboards Available?`
  (returns (Available :type Boolean))
  (return (`OnlineLeaderboardsSubsystem.IsSubsystemAvailable` (subsystem `OnlineLeaderboardsSubsystem`))))

(fn `Lobbies Available?`
  (returns (Available :type Boolean))
  (return (`OnlineLobbySubsystem.IsSubsystemAvailable` (subsystem `OnlineLobbySubsystem`))))

(fn `Parties Available?`
  (returns (Available :type Boolean))
  (return (`OnlinePartySubsystem.IsSubsystemAvailable` (subsystem `OnlinePartySubsystem`))))

(fn `Presence Available?`
  (returns (Available :type Boolean))
  (return (`OnlinePresenceSubsystem.IsSubsystemAvailable` (subsystem `OnlinePresenceSubsystem`))))

(fn `Sessions Available?`
  (returns (Available :type Boolean))
  (return (`OnlineSessionSubsystem.IsSubsystemAvailable` (subsystem `OnlineSessionSubsystem`))))

(fn `Stats Available?`
  (returns (Available :type Boolean))
  (return (`OnlineStatsSubsystem.IsSubsystemAvailable` (subsystem `OnlineStatsSubsystem`))))

(fn `TitleFile Available?`
  (returns (Available :type Boolean))
  (return (`OnlineTitleFileSubsystem.IsSubsystemAvailable` (subsystem `OnlineTitleFileSubsystem`))))

(fn `UserCloud Available?`
  (returns (Available :type Boolean))
  (return (`OnlineUserCloudSubsystem.IsSubsystemAvailable` (subsystem `OnlineUserCloudSubsystem`))))

(fn `UserConstructionScript`
  (`parent.UserConstructionScript`))

(fn `UserInfo Available?`
  (returns (Available :type Boolean))
  (return (`OnlineUserSubsystem.IsSubsystemAvailable` (subsystem `OnlineUserSubsystem`))))