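; Blueprint wrapper around an online friend in the ExampleOSS project, exposing user ID, ID type, real name and display name as strings.
; It builds a summary of wrapped subsystem accounts by parsing eosSynthetic user attributes.
; GetAvatar lazily starts a one-time fetch through the supplied FriendServices and immediately returns the cached avatar.
; HandleAvatarSet caches the result matching this friend, then unbinds from the fetch event.
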(fn `Get Avatar`
  (params (`Friend Services` :type "/Game/ExampleOSS/Common/BaseTasks/Friends/BaseFriendsServices Object Reference"))
  (returns (Texture :type "Texture2D Object Reference"))
  (if (not (`self.Is Fetching Avatar?`))
    (set `self.Is Fetching Avatar?` true)
    (add `/Game/ExampleOSS/Common/BaseTasks/Friends/BaseFriendsServices.On Avatar Fetched` `Friend Services` (`|CreateDelegate` :!event `Handle Avatar Set`))
    (set `self.Cached Friend Services` `Friend Services`)
    (`/Game/ExampleOSS/Common/BaseTasks/Friends/BaseFriendsServices.Fetch Avatar for Friend` `Friend Services` self))
  (return (`self.Cached Avatar`)))

(fn `Get Display Name`
  (returns (Value :type String))
  (return (`OnlineUserRef.GetDisplayName` (`self.Friend`))))

(fn `Get Real Name`
  (returns (Value :type String))
  (return (`OnlineUserRef.GetRealName` (`self.Friend`))))

(fn `Get User ID String`
  (returns (Value :type String))
  (return (`OnlineHelpers.Conv_FUniqueNetIdReplToString` (`OnlineUserRef.GetUserId` (`self.Friend`)))))

(fn `Get User ID Type`
  (returns (Value :type String))
  (return (`KismetStringLibrary.Conv_NameToString` (`OnlineHelpers.FUniqueNetIdGetType` (`OnlineUserRef.GetUserId` (`self.Friend`))))))

(fn `Get Wrapped Accounts Summary`
  (returns (Value :type String))
  (locals (WrapperText :type "Array of String"))
  (bind _friend (`self.Friend`))
  (bind (_found _returnvalue) (`OnlineUserRef.GetUserAttribute` (`self.Friend`) "eosSynthetic.subsystemNames"))
  (if _found
    (for _array_element (`KismetStringLibrary.ParseIntoArray` _returnvalue ",")
      (`KismetArrayLibrary.Array_Add` (`local.WrapperText`) (`KismetStringLibrary.Concat_StrStr` "subsystem: " _array_element " id: " (`.ReturnValue` (`OnlineUserRef.GetUserAttribute` _friend (`KismetStringLibrary.Concat_StrStr` "eosSynthetic.friend." _array_element ".id"))) " real name: " (`.ReturnValue` (`OnlineUserRef.GetUserAttribute` _friend (`KismetStringLibrary.Concat_StrStr` "eosSynthetic.friend." _array_element ".realName"))) " display name: " (`.ReturnValue` (`OnlineUserRef.GetUserAttribute` _friend (`KismetStringLibrary.Concat_StrStr` "eosSynthetic.friend." _array_element ".displayName"))))))
    (return (`KismetStringLibrary.JoinStringArray` (`local.WrapperText`) " \n"))
    (else
      (return ""))))

(fn `Handle Avatar Set`
  (params (Friend :type "/Game/ExampleOSS/Common/BaseTasks/Friends/BaseFriendReference Object Reference") (Avatar :type "Texture2D Object Reference"))
  (if (== Friend self)
    (set `self.Cached Avatar` Avatar)
    (remove `/Game/ExampleOSS/Common/BaseTasks/Friends/BaseFriendsServices.On Avatar Fetched` (`self.Cached Friend Services`) (`|CreateDelegate` :!event `Handle Avatar Set`))))