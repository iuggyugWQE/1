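; Short-lived task actor that joins an online party from a received invite.
; JoinParty casts the invite to BpPartyInviteReference and passes its party info and the first player controller's net ID to the online party subsystem.
; It reports success only on a Succeeded result, failure otherwise, then destroys itself.
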(event `self.Join Party`
  (params (Invite :type "/Game/ExampleOSS/Common/BaseTasks/Parties/BasePartyInviteReference Object Reference"))
  (bind (_localuserid _partyid _result) (`OnlinePartySubsystemJoinParty.JoinParty` (subsystem `OnlinePartySubsystem`) (`OnlineHelpers.GetControllerUniqueNetId` (`GameplayStatics.GetPlayerController` 0)) (`/Game/ExampleOSS/Blueprints/Parties/BpPartyInviteReference.Party Invite` (cast `/Game/ExampleOSS/Blueprints/Parties/BpPartyInviteReference` Invite :!pure true)))
    (:`OnCallFailed`
      (`self.On Complete` false))
    (:`OnJoinPartyComplete`
      (`self.On Complete` (`|EnumEquality` _result "Succeeded"))))
  (`self.K2_DestroyActor`))

(fn `UserConstructionScript`
  (`parent.UserConstructionScript`))