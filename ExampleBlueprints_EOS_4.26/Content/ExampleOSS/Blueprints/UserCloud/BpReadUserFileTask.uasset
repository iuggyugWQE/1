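; Short-lived task actor in the OSS example that reads one user cloud file for the first player controller's user.
; ReadUserFile takes a file entry, starts an async read through the Online User Cloud subsystem, then fetches the contents and converts them to a string.
; It fires OnComplete with a success flag and the text, or an empty string on any failure, then destroys itself.
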(event `self.Read User File`
  (params (File :type "/Game/ExampleOSS/Common/BaseTasks/UserCloud/BaseFileEntry Object Reference"))
  (bind _returnvalue (subsystem `OnlineUserCloudSubsystem`))
  (bind (_file_data_hash _file_data_hashtype _file_data_dlname _file_data_filename) (break `CloudFileHeaderBP` (`/Game/ExampleOSS/Blueprints/UserCloud/BpFileEntry.File Data` (cast `/Game/ExampleOSS/Blueprints/UserCloud/BpFileEntry` File :!pure true))))
  (bind (_bwassuccessful _userid _filename) (`OnlineUserCloudSubsystemReadUserFile.ReadUserFile` _returnvalue (`OnlineHelpers.GetControllerUniqueNetId` (`GameplayStatics.GetPlayerController` 0)) _file_data_filename)
    (:`OnCallFailed`
      (`self.On Complete` false :!label _label))
    (:`OnReadUserFileComplete`
      (if _bwassuccessful
        (bind (_filecontents _returnvalue_2) (`OnlineUserCloudSubsystem.GetFileContents` _returnvalue _userid _filename))
        (if _returnvalue_2
          (bind _returnvalue_3 (`OnlineHelpers.ReadFileDataAsString` _filecontents))
          (`self.On Complete` true _returnvalue_3)
          (else
            (goto _label)))
        (else
          (goto _label)))))
  (`self.K2_DestroyActor`))

(fn `UserConstructionScript`
  (`parent.UserConstructionScript`))