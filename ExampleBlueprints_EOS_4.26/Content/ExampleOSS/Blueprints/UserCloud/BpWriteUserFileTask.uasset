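; Task actor that writes a string to a named user cloud file through the Online User Cloud subsystem.
; It converts the text to file data and writes it asynchronously under the first player controller's unique net ID.
; It fires OnComplete with success or failure, treating failed calls and cancellations as failure, then destroys itself.
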(event `self.Write User File`
  (params (`File Name` :type String) (`File Data` :type String))
  (bind _returnvalue (`OnlineHelpers.CreateFileDataFromString` `File Data`))
  (bind _bwassuccessful (`OnlineUserCloudSubsystemWriteUserFile.WriteUserFile` (subsystem `OnlineUserCloudSubsystem`) (`OnlineHelpers.GetControllerUniqueNetId` (`GameplayStatics.GetPlayerController` 0)) `File Name` _returnvalue)
    (:`OnCallFailed`
      (`self.On Complete` false :!label _label))
    (:`OnWriteUserFileComplete`
      (if _bwassuccessful
        (`self.On Complete` true)
        (else
          (goto _label))))
    (:`OnWriteUserFileCanceled`
      (goto _label)))
  (`self.K2_DestroyActor`))

(fn `UserConstructionScript`
  (`parent.UserConstructionScript`))