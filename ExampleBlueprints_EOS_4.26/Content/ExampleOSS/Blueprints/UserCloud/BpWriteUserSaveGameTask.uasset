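; An actor Blueprint task that writes a SaveGame to the online user cloud for the first player controller's user.
; WriteUserFile serializes the SaveGame into file data and sends it to the Online User Cloud subsystem under the given file name.
; Completion reports success or failure through CallOnComplete, treating a failed call or cancellation as failure, then the actor destroys itself.
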(event `self.Write User File`
  (params (`File Name` :type String) (`Save Game` :type "/Game/ExampleOSS/Common/BaseTasks/UserCloud/ExampleSaveGame Object Reference"))
  (bind _returnvalue (`OnlineHelpers.CreateFileDataFromSaveGame` `Save Game`))
  (bind _bwassuccessful (`OnlineUserCloudSubsystemWriteUserFile.WriteUserFile` (subsystem `OnlineUserCloudSubsystem`) (`OnlineHelpers.GetControllerUniqueNetId` (`GameplayStatics.GetPlayerController` 0)) `File Name` _returnvalue)
    (:`OnCallFailed`
      (`self.On Complete` false :!label _label))
    (:`OnWriteUserFileComplete`
      (if _bwassuccessful
        (`self.On Complete` true)
        (else
          (goto _label))))
    (:`OnWriteUserFileCanceled`
      (goto _label)))
  (`self.K2_DestroyActor`))

(fn `UserConstructionScript`
  (`parent.UserConstructionScript`))