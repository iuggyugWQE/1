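; Task actor that connects the first local player to an existing online lobby by ID through the online lobby subsystem.
; On success it wraps the returned lobby in a BpLobbyRef, adds it to the lobby services' JoinedLobbies and reports it through CallOnComplete.
; A failed call or unsuccessful result reports failure instead.
; The actor is single-use and destroys itself after either outcome.
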(event `self.Connect Lobby`
  (params (`Lobby Id` :type "/Game/ExampleOSS/Common/BaseTasks/Lobbies/BaseLobbyIdRef Object Reference") (`Lobby Services` :type "/Game/ExampleOSS/Common/BaseTasks/Lobbies/BaseLobbyServices Object Reference"))
  (bind (_error _userid _lobby) (`OnlineLobbySubsystemConnectLobby.ConnectLobby` (subsystem `OnlineLobbySubsystem`) (`OnlineHelpers.GetControllerUniqueNetId` (`GameplayStatics.GetPlayerController` 0)) (`/Game/ExampleOSS/Blueprints/Lobbies/BpLobbyIdRef.Lobby Id` (cast `/Game/ExampleOSS/Blueprints/Lobbies/BpLobbyIdRef` `Lobby Id` :!pure true)))
    (:`OnCallFailed`
      (`self.On Complete` false :!label _label))
    (:`OnLobbyCreateOrConnectComplete`
      (if (break `OnlineErrorInfo` _error)
        (bind _returnvalue (`|GenericCreateObject` "/Game/ExampleOSS/Blueprints/Lobbies/BpLobbyRef.BpLobbyRef_C" `Lobby Services` _lobby))
        (`KismetArrayLibrary.Array_Add` (`/Game/ExampleOSS/Blueprints/Lobbies/BpLobbyServices.Joined Lobbies` (cast `/Game/ExampleOSS/Blueprints/Lobbies/BpLobbyServices` `Lobby Services` :!pure true)) _returnvalue)
        (`self.On Complete` true _returnvalue)
        (else
          (goto _label)))))
  (`self.K2_DestroyActor`))

(fn `UserConstructionScript`
  (`parent.UserConstructionScript`))