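; BpDisconnectLobbyTask is a one-shot task actor that disconnects the first local player from an online lobby.
; Its DisconnectLobby event unwraps the BpLobbyIdRef and runs the async DisconnectLobby call on the online lobby subsystem.
; On success it reports completion and removes the lobby from BpLobbyServices' joined lobbies; either failure path reports failure.
; The actor destroys itself once the operation finishes, whatever the result.
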(event `self.Disconnect Lobby`
  (params (`Lobby Id` :type "/Game/ExampleOSS/Common/BaseTasks/Lobbies/BaseLobbyIdRef Object Reference") (`Lobby Services` :type "/Game/ExampleOSS/Common/BaseTasks/Lobbies/BaseLobbyServices Object Reference"))
  (bind _error (`OnlineLobbySubsystemDisconnectLobby.DisconnectLobby` (subsystem `OnlineLobbySubsystem`) (`OnlineHelpers.GetControllerUniqueNetId` (`GameplayStatics.GetPlayerController` 0)) (`/Game/ExampleOSS/Blueprints/Lobbies/BpLobbyIdRef.Lobby Id` (cast `/Game/ExampleOSS/Blueprints/Lobbies/BpLobbyIdRef` `Lobby Id` :!pure true)))
    (:`OnCallFailed`
      (`self.On Complete` false `Lobby Id` :!label _label))
    (:`OnLobbyOperationComplete`
      (if (break `OnlineErrorInfo` _error)
        (`self.On Complete` true `Lobby Id`)
        (`/Game/ExampleOSS/Blueprints/Lobbies/BpLobbyServices.Remove Joined Lobby` (cast `/Game/ExampleOSS/Blueprints/Lobbies/BpLobbyServices` `Lobby Services` :!pure true) (cast `/Game/ExampleOSS/Blueprints/Lobbies/BpLobbyIdRef` `Lobby Id` :!pure true))
        (else
          (goto _label)))))
  (`self.K2_DestroyActor`))

(fn `UserConstructionScript`
  (`parent.UserConstructionScript`))