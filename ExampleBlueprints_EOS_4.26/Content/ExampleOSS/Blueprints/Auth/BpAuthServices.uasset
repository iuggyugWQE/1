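; Auth helper Blueprint in the OSS example that exposes the sign-in state and account details of local user 0.
; Each query reads the Online Identity subsystem for login status, nickname, user ID, or user and auth attributes such as Epic account ID, Product User ID and link eligibility.
; Account queries return false or empty when signed out, except the unguarded user ID getter.
; Dynamic config changes are hard-coded as unsupported, and the event graph is empty.
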(fn `Can Link To Epic Games Account?`
  (returns (`Can Link?` :type Boolean))
  (bind _returnvalue (subsystem `OnlineIdentitySubsystem`))
  (if (`self.Is Signed In?`)
    (return (`KismetStringLibrary.EqualEqual_StrStr` (`.ReturnValue` (`UserOnlineAccountRef.GetAuthAttribute` (`OnlineIdentitySubsystem.GetUserAccount` _returnvalue (`OnlineIdentitySubsystem.GetUniquePlayerId` _returnvalue 0)) "epic.canLink")) "true"))
    (else
      (return false))))

(fn `Get Epic Account ID`
  (returns (`Epic ID` :type String))
  (bind _returnvalue (subsystem `OnlineIdentitySubsystem`))
  (if (`self.Is Signed In?`)
    (return (`.ReturnValue` (`OnlineUserRef.GetUserAttribute` (`OnlineIdentitySubsystem.GetUserAccount` _returnvalue (`OnlineIdentitySubsystem.GetUniquePlayerId` _returnvalue 0)) "epicAccountId")))
    (else
      (return ""))))

(fn `Get Logged In Auth Attribute`
  (params (`Attribute Name` :type String))
  (returns (Value :type String))
  (bind _returnvalue (subsystem `OnlineIdentitySubsystem`))
  (if (`self.Is Signed In?`)
    (return (`.ReturnValue` (`UserOnlineAccountRef.GetAuthAttribute` (`OnlineIdentitySubsystem.GetUserAccount` _returnvalue (`OnlineIdentitySubsystem.GetUniquePlayerId` _returnvalue 0)) `Attribute Name`)))
    (else
      (return ""))))

(fn `Get Product User ID`
  (returns (PUID :type String))
  (bind _returnvalue (subsystem `OnlineIdentitySubsystem`))
  (if (`self.Is Signed In?`)
    (return (`.ReturnValue` (`OnlineUserRef.GetUserAttribute` (`OnlineIdentitySubsystem.GetUserAccount` _returnvalue (`OnlineIdentitySubsystem.GetUniquePlayerId` _returnvalue 0)) "productUserId")))
    (else
      (return ""))))

(fn `Get User Id`
  (returns (`User Id` :type "UniqueNetIdRepl Structure"))
  (return (`OnlineIdentitySubsystem.GetUniquePlayerId` (subsystem `OnlineIdentitySubsystem`) 0)))

(fn `Get Username`
  (returns (Username :type String))
  (bind _returnvalue (subsystem `OnlineIdentitySubsystem`))
  (if (`self.Is Signed In?`)
    (return (`OnlineIdentitySubsystem.GetPlayerNickname` _returnvalue (`OnlineIdentitySubsystem.GetUniquePlayerId` _returnvalue 0)))
    (else
      (return ""))))

(fn `Is Config Dynamically Changeable?`
  (returns (`Is Dynamic` :type Boolean))
  (return false))

(fn `Is Signed In with Epic Games Account?`
  (returns (`Signed in with Epic?` :type Boolean))
  (bind _returnvalue (subsystem `OnlineIdentitySubsystem`))
  (if (`self.Is Signed In?`)
    (return (`KismetStringLibrary.EqualEqual_StrStr` (`.ReturnValue` (`UserOnlineAccountRef.GetAuthAttribute` (`OnlineIdentitySubsystem.GetUserAccount` _returnvalue (`OnlineIdentitySubsystem.GetUniquePlayerId` _returnvalue 0)) "authenticatedWith")) "epic"))
    (else
      (return false))))

(fn `Is Signed In?`
  (returns (`Signed In?` :type Boolean))
  (return (`|EnumEquality` (`OnlineIdentitySubsystem.GetLoginStatus` (subsystem `OnlineIdentitySubsystem`) 0) "LoggedIn")))

(fn `UserConstructionScript`
  (`parent.UserConstructionScript`))