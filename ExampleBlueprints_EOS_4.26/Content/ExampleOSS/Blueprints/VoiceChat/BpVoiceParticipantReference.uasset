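; Voice chat participant reference that represents one player by name in the ExampleOSS voice chat.
; It reports whether that player is talking or muted by querying the VoiceUser held in BpVoiceServices with the player name.
; ToString returns the player name.
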(fn `Is Muted?`
  (returns (`Muted?` :type Boolean))
  (return (`VoiceChatUser.IsPlayerMuted` (`/Game/ExampleOSS/Blueprints/VoiceChat/BpVoiceChatServices.Voice User` (`self.Bp Voice Services`)) (`self.Player Name`))))

(fn `Is Speaking?`
  (returns (Speaking :type Boolean))
  (return (`VoiceChatUser.IsPlayerTalking` (`/Game/ExampleOSS/Blueprints/VoiceChat/BpVoiceChatServices.Voice User` (`self.Bp Voice Services`)) (`self.Player Name`))))

(fn `ToString`
  (returns (Value :type String))
  (return (`self.Player Name`)))