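; Voice chat service Blueprint that wraps the OnlineVoiceChatSubsystem for the game.
; On BeginPlay it creates a voice user, falling back to the primary one, and binds its device, channel and player events.
; Events print debug messages, with channel and participant changes also firing dispatchers.
; Functions expose status, devices as "name--id" strings that setters split to recover the ID, and channels and players wrapped in newly constructed reference objects.
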(event `self.ReceiveBeginPlay`
  (bind _returnvalue (subsystem `OnlineVoiceChatSubsystem`))
  (bind _voice_user (`self.Voice User`))
  (bind _returnvalue_2 (`OnlineVoiceChatSubsystem.CreateUser` _returnvalue))
  (`/Engine/EditorBlueprintResources/StandardMacros.IsValid` _returnvalue_2
    (:`Is Valid`
      (set `self.Voice User` _returnvalue_2))
    (:`Is Not Valid`
      (set `self.Voice User` (`OnlineVoiceChatSubsystem.PrimaryVoiceUser` _returnvalue))))
  (`|ExecutionSequence`
    (:`then_0`
      (add `VoiceChatUser.OnVoiceChatAvailableAudioDevicesChanged` _voice_user (delegate `Audio Devices Changed`)))
    (:`then_1`
      (add `VoiceChatUser.OnVoiceChatChannelJoined` _voice_user (delegate `Voice Chat Channel Joined`)))
    (:`then_2`
      (add `VoiceChatUser.OnVoiceChatChannelExited` _voice_user (delegate `Voice Chat Channel Exited`)))
    (:`then_3`
      (add `VoiceChatUser.OnVoiceChatPlayerAdded` _voice_user (delegate `Voice Chat Player Added`)))
    (:`then_4`
      (add `VoiceChatUser.OnVoiceChatPlayerRemoved` _voice_user (delegate `Voice Chat Player Removed`)))
    (:`then_5`
      (add `VoiceChatUser.OnVoiceChatPlayerMuteUpdated` _voice_user (delegate `Voice Chat Player Mute Updated`)))
    (:`then_6`
      (add `VoiceChatUser.OnVoiceChatPlayerTalkingUpdated` _voice_user (delegate `Voice Chat Player Talking Updated`)))))

(event `Audio Devices Changed`
  (`KismetSystemLibrary.PrintString` "Voice Chat: Audio devices changed"))

(event `Voice Chat Channel Joined`
  (params (ChannelName :type String))
  (`KismetSystemLibrary.PrintString` (`KismetStringLibrary.Concat_StrStr` "Voice Chat: Channel joined: " ChannelName))
  (`self.Joined Channels Changed`))

(event `Voice Chat Channel Exited`
  (params (ChannelName :type String) (Reason :type "VoiceChatResultBP Structure"))
  (`KismetSystemLibrary.PrintString` (`KismetStringLibrary.Concat_StrStr` "Voice Chat: Channel exited: " ChannelName " Reason: " (`|GetEnumeratorNameAsString` Reason_ResultCode)))
  (`self.Joined Channels Changed`))

(event `Voice Chat Player Added`
  (params (ChannelName :type String) (PlayerName :type String))
  (`KismetSystemLibrary.PrintString` (`KismetStringLibrary.Concat_StrStr` "Voice Chat: Player added in channel: " ChannelName " Player name: " PlayerName))
  (`self.Participants Changed`))

(event `Voice Chat Player Removed`
  (params (ChannelName :type String) (PlayerName :type String))
  (`KismetSystemLibrary.PrintString` (`KismetStringLibrary.Concat_StrStr` "Voice Chat: Player removed in channel: " ChannelName " Player name: " PlayerName))
  (`self.Participants Changed`))

(event `Voice Chat Player Mute Updated`
  (params (ChannelName :type String) (PlayerName :type String) (bIsMuted :type Boolean))
  (`KismetSystemLibrary.PrintString` (`KismetStringLibrary.Concat_StrStr` "Voice Chat: Player mute changed in channel: " ChannelName " Player name: " PlayerName " Muted: " (`KismetStringLibrary.Conv_BoolToString` bIsMuted))))

(event `Voice Chat Player Talking Updated`
  (params (ChannelName :type String) (PlayerName :type String) (bIsTalking :type Boolean))
  (`KismetSystemLibrary.PrintString` (`KismetStringLibrary.Concat_StrStr` "Voice Chat: Player talking changed in channel: " ChannelName " Player name: " PlayerName " Talking: " (`KismetStringLibrary.Conv_BoolToString` bIsTalking))))

(fn `Get Available Input Devices`
  (returns (Devices :type "Array of String"))
  (locals (Results :type "Array of String"))
  (bind _returnvalue (`VoiceChatUser.GetAvailableInputDeviceInfos` (`self.Voice User`)))
  (for _array_element _returnvalue
    (`KismetArrayLibrary.Array_Add` (`local.Results`) (`KismetStringLibrary.Concat_StrStr` (break `VoiceChatDeviceInfoBP` _array_element) " -- " (`.Id` (break `VoiceChatDeviceInfoBP` _array_element)))))
  (return (`local.Results`)))

(fn `Get Available Output Devices`
  (returns (Devices :type "Array of String"))
  (locals (Results :type "Array of String"))
  (bind _returnvalue (`VoiceChatUser.GetAvailableOutputDeviceInfos` (`self.Voice User`)))
  (for _array_element _returnvalue
    (`KismetArrayLibrary.Array_Add` (`local.Results`) (`KismetStringLibrary.Concat_StrStr` (break `VoiceChatDeviceInfoBP` _array_element) " -- " (`.Id` (break `VoiceChatDeviceInfoBP` _array_element)))))
  (return (`local.Results`)))

(fn `Get Current Input Device`
  (returns (Device :type String))
  (bind (_returnvalue_displayname _returnvalue_id) (break `VoiceChatDeviceInfoBP` (`VoiceChatUser.GetInputDeviceInfo` (`self.Voice User`))))
  (return (`KismetStringLibrary.Concat_StrStr` _returnvalue_displayname " -- " _returnvalue_id)))

(fn `Get Current Output Device`
  (returns (Device :type String))
  (bind (_returnvalue_displayname _returnvalue_id) (break `VoiceChatDeviceInfoBP` (`VoiceChatUser.GetOutputDeviceInfo` (`self.Voice User`))))
  (return (`KismetStringLibrary.Concat_StrStr` _returnvalue_displayname " -- " _returnvalue_id)))

(fn `Get Joined Channels`
  (returns (Channels :type "Array of /Game/ExampleOSS/Common/BaseTasks/VoiceChat/BaseVoiceChannelReference Object Reference"))
  (locals (Results :type "Array of /Game/ExampleOSS/Common/BaseTasks/VoiceChat/BaseVoiceChannelReference Object Reference"))
  (bind _returnvalue (`VoiceChatUser.GetChannels` (`self.Voice User`)))
  (for _array_element _returnvalue
    (bind _returnvalue_2 (`|GenericCreateObject` "/Game/ExampleOSS/Blueprints/VoiceChat/BpVoiceChannelReference.BpVoiceChannelReference_C" (`GameplayStatics.GetPlayerController` 0) _array_element))
    (`KismetArrayLibrary.Array_Add` (`local.Results`) _returnvalue_2))
  (return (`local.Results`)))

(fn `Get Logged In Player Name`
  (returns (`Player Name` :type String))
  (return (`VoiceChatUser.GetLoggedInPlayerName` (`self.Voice User`))))

(fn `Get Players In Channel`
  (params (Channel :type "/Game/ExampleOSS/Common/BaseTasks/VoiceChat/BaseVoiceChannelReference Object Reference"))
  (returns (Participants :type "Array of /Game/ExampleOSS/Common/BaseTasks/VoiceChat/BaseVoiceParticipantReference Object Reference"))
  (locals (Results :type "Array of /Game/ExampleOSS/Common/BaseTasks/VoiceChat/BaseVoiceParticipantReference Object Reference"))
  (bind _channel_name (`/Game/ExampleOSS/Blueprints/VoiceChat/BpVoiceChannelReference.Channel Name` (cast `/Game/ExampleOSS/Blueprints/VoiceChat/BpVoiceChannelReference` Channel :!pure true)))
  (bind _returnvalue (`VoiceChatUser.GetPlayersInChannel` (`self.Voice User`) _channel_name))
  (for _array_element _returnvalue
    (bind _returnvalue_2 (`|GenericCreateObject` "/Game/ExampleOSS/Blueprints/VoiceChat/BpVoiceParticipantReference.BpVoiceParticipantReference_C" (`GameplayStatics.GetPlayerController` 0) _channel_name _array_element self))
    (`KismetArrayLibrary.Array_Add` (`local.Results`) _returnvalue_2))
  (return (`local.Results`)))

(fn `Is Connected?`
  (returns (Connected :type Boolean))
  (return (`OnlineVoiceChatSubsystem.IsConnected` (subsystem `OnlineVoiceChatSubsystem`))))

(fn `Is Connecting?`
  (returns (Connecting :type Boolean))
  (return (`OnlineVoiceChatSubsystem.IsConnecting` (subsystem `OnlineVoiceChatSubsystem`))))

(fn `Is Logged In?`
  (returns (`Logged In` :type Boolean))
  (return (`VoiceChatUser.IsLoggedIn` (`self.Voice User`))))

(fn `Set Input Device`
  (params (Device :type String))
  (`VoiceChatUser.SetInputDeviceId` (`self.Voice User`) (`.RightS` (`KismetStringLibrary.Split` Device " -- " "IgnoreCase" "FromEnd"))))

(fn `Set Output Device`
  (params (Device :type String))
  (`VoiceChatUser.SetOutputDeviceId` (`self.Voice User`) (`.RightS` (`KismetStringLibrary.Split` Device " -- " "IgnoreCase" "FromEnd"))))

(fn `UserConstructionScript`
  (`parent.UserConstructionScript`))