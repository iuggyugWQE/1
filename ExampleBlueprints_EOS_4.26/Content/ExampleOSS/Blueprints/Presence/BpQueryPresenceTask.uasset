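; One-shot actor task in the ExampleOSS example that queries online presence, reported in its messages as presence information for friends.
; QueryPresence starts an async query on the online presence subsystem using the first player controller's unique net ID.
; It broadcasts OnComplete with success or failure, treating a failed call and an unsuccessful result alike, prints the outcome, then destroys itself.
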(event `self.Query Presence`
  (bind (_userid _bwassuccessful) (`OnlinePresenceSubsystemQueryPresence.QueryPresence` (subsystem `OnlinePresenceSubsystem`) (`OnlineHelpers.GetControllerUniqueNetId` (`GameplayStatics.GetPlayerController` 0)))
    (:`OnCallFailed`
      (`self.On Complete` false :!label _label)
      (`KismetSystemLibrary.PrintString` "Failed to fetch presence from friends."))
    (:`OnPresenceTaskComplete`
      (if _bwassuccessful
        (`self.On Complete` true)
        (`KismetSystemLibrary.PrintString` "Got presence information for friends!")
        (else
          (goto _label)))))
  (`self.K2_DestroyActor`))

(fn `UserConstructionScript`
  (`parent.UserConstructionScript`))