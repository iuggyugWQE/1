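; BpGetAvatarForFriendTask is a short-lived actor that fetches a friend's avatar through the online avatar subsystem.
; FetchFriendAvatar runs an async GetAvatar for the local player against the friend's user ID, with a Font Awesome user icon as default.
; Completion or call failure reports the resulting texture or fallback icon through CallOnAvatarFetched, then the actor destroys itself.
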(event `self.Fetch Friend Avatar`
  (params (Friend :type "/Game/ExampleOSS/Common/BaseTasks/Friends/BaseFriendReference Object Reference"))
  (bind (_bwassuccessful _resulttexture) (`OnlineAvatarSubsystemGetAvatar.GetAvatar` (subsystem `OnlineAvatarSubsystem`) (`OnlineHelpers.GetControllerUniqueNetId` (`GameplayStatics.GetPlayerController` 0)) (`OnlineUserRef.GetUserId` (`/Game/ExampleOSS/Blueprints/Friends/BpFriendReference.Friend` (cast `/Game/ExampleOSS/Blueprints/Friends/BpFriendReference` Friend :!pure true))) "/Game/ExampleOSS/Common/UIComponents/FontAwesomeUserIcon.FontAwesomeUserIcon")
    (:`OnCallFailed`
      (`self.On Avatar Fetched` Friend "/Game/ExampleOSS/Common/UIComponents/FontAwesomeUserIcon.FontAwesomeUserIcon"))
    (:`OnGetAvatarComplete`
      (`self.On Avatar Fetched` Friend _resulttexture)))
  (`self.K2_DestroyActor`))

(fn `UserConstructionScript`
  (`parent.UserConstructionScript`))