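; One-shot actor task that logs the first local player into voice chat in the OSS example.
; On VoiceLogin, it runs an async Login on the VoiceUser from BpVoiceChatServices.
; The platform ID and player name both derive from the Online Identity subsystem's unique ID for player 0, with the stringified ID serving as the name.
; It reports success or failure through CallOnComplete, then destroys itself.
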(event `self.Voice Login`
  (params (`Voice Chat Services` :type "/Game/ExampleOSS/Common/BaseTasks/VoiceChat/BaseVoiceChatServices Object Reference"))
  (bind _returnvalue (subsystem `OnlineIdentitySubsystem`))
  (bind _returnvalue_2 (`OnlineIdentitySubsystem.GetUniquePlayerId` _returnvalue 0))
  (bind (_playername _result) (`VoiceChatUserLogin.Login` (`/Game/ExampleOSS/Blueprints/VoiceChat/BpVoiceChatServices.Voice User` (cast `/Game/ExampleOSS/Blueprints/VoiceChat/BpVoiceChatServices` `Voice Chat Services` :!pure true)) (`OnlineIdentitySubsystem.GetPlatformUserIdFromUniqueNetId` _returnvalue _returnvalue_2) (`OnlineHelpers.Conv_FUniqueNetIdReplToString` _returnvalue_2))
    (:`OnCallFailed`
      (`self.On Complete` false))
    (:`OnVoiceChatLoginComplete`
      (`self.On Complete` (break `VoiceChatResultBP` _result))))
  (`self.K2_DestroyActor`))

(fn `UserConstructionScript`
  (`parent.UserConstructionScript`))