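; An example Blueprint task actor that reads local user 0's online friends list through the OnlineFriendsSubsystem.
; It runs an async ReadFriendsList, gets the cached list, and wraps each friend in a BpFriendReference.
; It reports success with those results, or failure with an empty array, then destroys itself.
; An unconnected branch shows how to inject a derived emulated friend into the results.
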(event `self.Read and Get Friends`
  (bind (_localusernum _bwassuccessful) (`OnlineFriendsSubsystemReadFriendsList.ReadFriendsList` (subsystem `OnlineFriendsSubsystem`))
    (:`OnCallFailed`
      (`self.On Complete` false (`|MakeArray`) :!label _label)
      (`self.K2_DestroyActor`))
    (:`OnReadFriendsListComplete`
      (if _bwassuccessful
        (bind (_outfriends _returnvalue) (`OnlineFriendsSubsystem.GetFriendsList` (subsystem `OnlineFriendsSubsystem`) 0 ""))
        (if _returnvalue
          (bind _output_get (set `self.Results` (`|MakeArray`)))
          ;[1 1 1] Add the actual friends
          (for _array_element _outfriends
            (bind _returnvalue_2 (`|GenericCreateObject` (`GameplayStatics.GetPlayerController` 0) "/Game/ExampleOSS/Blueprints/Friends/BpFriendReference.BpFriendReference_C" _array_element))
            (`KismetArrayLibrary.Array_Add` (`self.Results`) _returnvalue_2))
          (`self.On Complete` true (`self.Results`))
          (`self.K2_DestroyActor`)
          (else
            (goto _label)))
        (else
          (goto _label))))))

(fn `UserConstructionScript`
  (`parent.UserConstructionScript`))