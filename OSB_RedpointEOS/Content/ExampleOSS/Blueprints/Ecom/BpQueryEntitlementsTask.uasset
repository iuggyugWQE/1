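; One-shot task actor that queries the local player's entitlements through the Online Subsystem entitlements interface, in an ExampleOSS e-commerce example.
; On success it reads all entitlements for the returned user and namespace and wraps each in a BpEntitlementReference object.
; It reports success with that list, or failure with an empty one, through OnQueryEntitlementsComplete, then destroys itself.
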(event `self.Query Entitlements`
  (bind _returnvalue (subsystem `OnlineEntitlementsSubsystem`))
  (bind (_bwassuccessful _userid _namespace) (`OnlineEntitlementsSubsystemQueryEntitlements.QueryEntitlements` _returnvalue (`OnlineHelpers.GetControllerUniqueNetId` (`GameplayStatics.GetPlayerController` 0)))
    (:`OnCallFailed`
      (`KismetSystemLibrary.PrintString` "Entitlement fetch failed." :!label _label)
      (`self.On Query Entitlements Complete` false (`|MakeArray`))
      (`self.K2_DestroyActor`))
    (:`OnQueryEntitlementsComplete`
      (if _bwassuccessful
        (bind _outuserentitlements (`OnlineEntitlementsSubsystem.GetAllEntitlements` _returnvalue _userid _namespace))
        (for _array_element _outuserentitlements
          (bind _returnvalue_2 (`|GenericCreateObject` (`GameplayStatics.GetPlayerController` 0) "/Game/ExampleOSS/Blueprints/Ecom/BpEntitlementReference.BpEntitlementReference_C" _array_element))
          (`KismetArrayLibrary.Array_Add` (`self.Results`) _returnvalue_2))
        (`KismetSystemLibrary.PrintString` (`KismetStringLibrary.Concat_StrStr` "Fetched " (`KismetStringLibrary.Conv_IntToString` (`KismetArrayLibrary.Array_Length` (`self.Results`))) " entitlements."))
        (`self.On Query Entitlements Complete` true (`self.Results`))
        (`self.K2_DestroyActor`)
        (else
          (goto _label))))))

(fn `UserConstructionScript`
  (`parent.UserConstructionScript`))