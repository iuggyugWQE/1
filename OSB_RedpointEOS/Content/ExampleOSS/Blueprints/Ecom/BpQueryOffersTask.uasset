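; A Blueprint task actor that queries the online store's offers for the first local player through the OnlineStoreV2 subsystem.
; On success it wraps each returned offer in a BpOfferReference object and reports the list through an OnQueryOffersComplete dispatcher.
; Failed calls and unsuccessful queries print the error and report an empty result.
; The actor destroys itself once the query resolves.
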(event `self.Query Offers`
  (bind _returnvalue (subsystem `OnlineStoreV2Subsystem`))
  (bind _results (`self.Results`))
  (bind (_bwassuccessful _offerids _error) (`OnlineStoreV2SubsystemQueryOffersByFilter.QueryOffersByFilter` _returnvalue (`OnlineHelpers.GetControllerUniqueNetId` (`GameplayStatics.GetPlayerController` 0)))
    (:`OnCallFailed`
      (`KismetSystemLibrary.PrintString` _error :!label _label)
      (`self.On Query Offers Complete` false (`|MakeArray`))
      (`self.K2_DestroyActor`))
    (:`OnQueryOnlineStoreOffersComplete`
      (if _bwassuccessful
        (bind _outoffers (`OnlineStoreV2Subsystem.GetOffers` _returnvalue))
        (for _array_element _outoffers
          (bind _returnvalue_2 (`|GenericCreateObject` (`GameplayStatics.GetPlayerController` 0) "/Game/ExampleOSS/Blueprints/Ecom/BpOfferReference.BpOfferReference_C" _array_element))
          (`KismetArrayLibrary.Array_Add` (`self.Results`) _returnvalue_2))
        (`self.On Query Offers Complete` true _results)
        (`KismetSystemLibrary.PrintString` (`KismetStringLibrary.Concat_StrStr` "Obtained " (`KismetStringLibrary.Conv_IntToString` (`KismetArrayLibrary.Array_Length` _results)) " offers successfully from API."))
        (`self.K2_DestroyActor`)
        (else
          (goto _label))))))

(fn `UserConstructionScript`
  (`parent.UserConstructionScript`))