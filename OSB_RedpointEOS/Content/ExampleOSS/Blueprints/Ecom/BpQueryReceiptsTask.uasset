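; Example task actor that queries a player's purchase receipts through the Online Subsystem purchase interface.
; QueryReceipts starts an async query for player controller 0's unique net ID, with receipt restoring enabled.
; A failed call or unsuccessful result prints the error, calls OnQueryReceiptsComplete with failure and no receipts, then destroys the actor.
; The successful branch is unwired, so it neither reports receipts nor destroys the actor.
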(event `self.Query Receipts`
  (bind _result (`OnlinePurchaseSubsystemQueryReceipts.QueryReceipts` (subsystem `OnlinePurchaseSubsystem`) (`OnlineHelpers.GetControllerUniqueNetId` (`GameplayStatics.GetPlayerController` 0)) true)
    (:`OnCallFailed`
      (`KismetSystemLibrary.PrintString` (`KismetTextLibrary.Conv_TextToString` (`.ErrorMessage` (break `OnlineErrorInfo` _result))) :!label _label)
      (`self.On Query Receipts Complete` false (`|MakeArray`))
      (`self.K2_DestroyActor`))
    (:`OnQueryReceiptsComplete`
      (if (not (break `OnlineErrorInfo` _result))
        (goto _label)))))

(fn `UserConstructionScript`
  (`parent.UserConstructionScript`))