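; BpOfferReference is a wrapper around a single store offer in the ExampleOSS e-commerce sample.
; It holds an Offer and exposes getters for its ID, current price and title, each forwarding directly to that offer.
; The current price getter returns the offer's display price.
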(fn `Get Current Price`
  (returns (`Display Price` :type Text))
  (return (`OnlineStoreOffer.GetDisplayPrice` (`self.Offer`))))

(fn `Get Id`
  (returns (Id :type String))
  (return (`OnlineStoreOffer.GetOfferId` (`self.Offer`))))

(fn `Get Title`
  (returns (Title :type Text))
  (return (`OnlineStoreOffer.GetTitle` (`self.Offer`))))