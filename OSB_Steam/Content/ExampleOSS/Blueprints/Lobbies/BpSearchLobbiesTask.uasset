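; Short-lived task actor that searches for online lobbies through the Online Subsystem lobby interface in the OSS example project.
; It searches as the first local player with a "Type equals Lobby" filter, included because subsystems like EOS require at least one.
; Each found lobby ID is wrapped in a BpLobbyIdRef object and returned through CallOnComplete, with failures returning an empty list.
; The actor destroys itself after reporting either result.
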(event `self.Search Lobbies`
  (bind (_error _userid _lobbies) (`OnlineLobbySubsystemSearch.Search` (subsystem `OnlineLobbySubsystem`) (`OnlineHelpers.GetControllerUniqueNetId` (`GameplayStatics.GetPlayerController` 0)) (make `OnlineLobbySearchQueryBP` (`|MakeArray` (make `OnlineLobbySearchQueryFilterBP` "Type" (make `VariantDataBP` "String" false 0 0.0 0 "Lobby")))))
    (:`OnCallFailed`
      (`self.On Complete` false (`|MakeArray`) :!label _label)
      (`self.K2_DestroyActor`))
    (:`OnLobbySearchComplete`
      (if (break `OnlineErrorInfo` _error)
        (for _array_element _lobbies
          (bind _returnvalue (`|GenericCreateObject` "/Game/ExampleOSS/Blueprints/Lobbies/BpLobbyIdRef.BpLobbyIdRef_C" self _array_element))
          (`KismetArrayLibrary.Array_Add` (`self.Results`) _returnvalue))
        (`self.On Complete` true (`self.Results`))
        (`self.K2_DestroyActor`)
        (else
          (goto _label))))))

(fn `UserConstructionScript`
  (`parent.UserConstructionScript`))