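; Example session service Blueprint that wraps the online session subsystem for joining and querying sessions.
; On BeginPlay it binds accepted overlay invites, joins that session and signals that map travel is required.
; Helpers resolve connect strings and report the local session's ID and registered players, which only the host sees.
; Party leaders make members follow by writing a randomly prefixed session ID into party data, so each request registers as new.
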(event `self.ReceiveBeginPlay`
  (add `OnlineSessionSubsystem.OnSessionUserInviteAccepted` (subsystem `OnlineSessionSubsystem`) (delegate `Accepted Invite to Session`)))

(event `Accepted Invite to Session`
  (params (bWasSuccessful :type Boolean) (ControllerId :type Integer) (UserId :type "UniqueNetIdRepl Structure") (InviteResult :type "OnlineSessionSearchResultBP Structure"))
  ;[0 0 0] When the user accepts an invite to a session in the overlay, we have to handle it and join the session in-game. After joining, we tell the common example code to connect to the server.
  (bind (_sessionname _result) (`OnlineSessionSubsystemJoinSession.JoinSession` (subsystem `OnlineSessionSubsystem`) (`OnlineHelpers.GetControllerUniqueNetId` (`GameplayStatics.GetPlayerController` 0)) (`KismetStringLibrary.Conv_StringToName` (`.SessionId` (break `OnlineSessionBP` (`.Session` (break `OnlineSessionSearchResultBP` InviteResult))))) InviteResult)
    (:`OnCallFailed`
      (`KismetSystemLibrary.PrintString` "Could not join session after accepting session invite!" :!label _label))
    (:`OnJoinSessionComplete`
      (if (`|EnumEquality` _result "Success")
        (`self.Session Joined Map Travel Required` _sessionname)
        (else
          (goto _label))))))

(fn `Begin Recording Replay`
  (params (`Game Mode` :type "GameModeBase Object Reference")))

(fn `Get Current Session Id`
  (returns (`Session Id` :type String))
  (bind _returnvalue (`OnlineSessionSubsystem.GetNamedSession` (subsystem `OnlineSessionSubsystem`) "MyLocalSessionName"))
  ;[0 0 0] A session by the specified name might not exist, so call IsValid to see if we got a session. If we did, call GetValue to get the actual data.
  (`/Engine/EditorBlueprintResources/StandardMacros.IsValid` _returnvalue
    (:`Is Valid`
      (return (`.SessionId` (break `NamedOnlineSessionBP` (`NamedOnlineSession.GetValue` _returnvalue)))))
    (:`Is Not Valid`
      (return ""))))

(fn `Get Players in Session`
  (returns (Players :type "Array of String"))
  (locals (Results :type "Array of String"))
  (bind _returnvalue (`OnlineSessionSubsystem.GetNamedSession` (subsystem `OnlineSessionSubsystem`) "MyLocalSessionName"))
  ;[0 0 0] A session by the specified name might not exist, so call IsValid to see if we got a session. If we did, call GetValue to get the actual data.
  (`/Engine/EditorBlueprintResources/StandardMacros.IsValid` _returnvalue
    (:`Is Valid`
      (set `local.Results` (`|MakeArray`))
      (bind (_sessionname _bhosting _localownerid _registeredplayers _sessionstate _owninguserid) (break `NamedOnlineSessionBP` (`NamedOnlineSession.GetValue` _returnvalue)))
      ;[0 0 0] Get the registered players from the session. Sessions are not synchronised between the host and clients, so the list of registered players is only visible to the session host.
      ;
      ; If you want a list of players to be visible to clients, you should use Unreal replication (i.e. get the host to store a list of players in the GameState, replicate it, and have clients read from it while they're connected to the server).
      (for _array_element _registeredplayers
        (`KismetArrayLibrary.Array_Add` (`local.Results`) (`KismetStringLibrary.Concat_StrStr` "(" (`KismetMathLibrary.SelectString` "host" "client" (== _array_element _owninguserid)) "): " (`OnlineHelpers.Conv_FUniqueNetIdReplToString` _array_element))))
      (return (`local.Results`)))
    (:`Is Not Valid`
      (return (`|MakeArray`)))))

(fn `Get Resolved Connect String from Search Result`
  (params (`Search Result` :type "/Game/ExampleOSS/Common/BaseTasks/Session/BaseSessionReference Object Reference"))
  (returns (`Connection String` :type String))
  (return (`.OutConnectInfo` (`OnlineHelpers.GetResolvedConnectStringBySearchResult` (subsystem `OnlineSessionSubsystem`) (`/Game/ExampleOSS/Blueprints/Session/BpSessionReference.Session` (cast `/Game/ExampleOSS/Blueprints/Session/BpSessionReference` `Search Result` :!pure true)) "GamePort"))))

(fn `Get Resolved Connect String from Session Name`
  (params (`Session Name` :type Name))
  (returns (`Connection String` :type String))
  (return (`.OutConnectInfo` (`OnlineHelpers.GetResolvedConnectStringByName` (subsystem `OnlineSessionSubsystem`) `Session Name` "GamePort"))))

(fn `Get User Id from Unique Net Id`
  (params (`User Id Repl` :type "UniqueNetIdRepl Structure"))
  (returns (Result :type String))
  (return (`OnlineHelpers.Conv_FUniqueNetIdReplToString` `User Id Repl`)))

(fn `Request Party Members Follow Leader`
  (params (`Session Name` :type Name))
  (bind _returnvalue (subsystem `OnlinePartySubsystem`))
  (bind _returnvalue_2 (`OnlineHelpers.GetControllerUniqueNetId` (`GameplayStatics.GetPlayerController` 0)))
  (bind _returnvalue_3 (`OnlineSessionSubsystem.GetNamedSession` (subsystem `OnlineSessionSubsystem`) `Session Name`))
  ;[0 0 0] A session by the specified name might not exist, so call IsValid to see if we got a session. If we did, call GetValue to get the actual data.
  (`/Engine/EditorBlueprintResources/StandardMacros.IsValid` _returnvalue_3
    (:`Is Valid`
      ;[0 0 0] Iterate over the joined parties that we're in, and if we're the leader, update the party data. Other members will see the party data change via an event, and that's how they get the session follow string. Take a look in BeginPlay of the party class (BpPartyServices) to see how to handle responding to the party data change event.
      (for _array_element (`OnlinePartySubsystem.GetJoinedParties` _returnvalue _returnvalue_2)
        ;[0 0 0] Check if we're the leader of the party...
        (bind _returnvalue_4 (`Party.GetLeaderId` (`OnlinePartySubsystem.GetParty` _returnvalue _returnvalue_2 _array_element)))
        (if (== _returnvalue_4 (`OnlineHelpers.GetControllerUniqueNetId` (`GameplayStatics.GetPlayerController` 0)))
          ;[0 0 0] When you get party data with GetPartyData, it's read only. That's because it's the cached party data you currently have.
          ;
          ; When you want to update a party, you first need to create a writable copy of the party data using "Create Modifiable Party Data". You can then set or remove attributes on it, and then pass it into UpdatePartyData.
          (bind _returnvalue_5 (`OnlineHelpers.CreateMutablePartyData` (`OnlinePartySubsystem.GetPartyData` _returnvalue _returnvalue_2 _array_element "None")))
          (`MutablePartyData.SetAttribute` _returnvalue_5 "SessionFollowString" (make `VariantDataBP` "String" false 0 0.0 0 (`KismetStringLibrary.Concat_StrStr` (`KismetStringLibrary.Conv_IntToString` (`KismetMathLibrary.RandomInteger` 0)) "|" (`.SessionId` (break `NamedOnlineSessionBP` (`NamedOnlineSession.GetValue` _returnvalue_3))))))
          ;[0 0 0] Now call UpdatePartyData. This is an asynchronous operation - if you want to know when the party data has actually propagated to other clients, listen for the OnPartyDataUpdated event (you'll get an event for your own update).
          (`OnlinePartySubsystem.UpdatePartyData` (subsystem `OnlinePartySubsystem`) (`OnlineHelpers.GetControllerUniqueNetId` (`GameplayStatics.GetPlayerController` 0)) _array_element "None" _returnvalue_5)))
      (return))
    (:`Is Not Valid`
      (return))))

(fn `UserConstructionScript`
  (`parent.UserConstructionScript`))