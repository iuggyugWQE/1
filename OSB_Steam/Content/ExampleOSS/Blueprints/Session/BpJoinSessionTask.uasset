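; Actor task that joins an online session through the OnlineSessionSubsystem for the first local player.
; JoinSession casts the passed reference to BpSessionReference and runs an async join using that session and name.
; It reports success only when the join result is Success, reports failure if the call fails, then destroys itself.
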(event `self.Join Session`
  (params (`Session Name` :type Name) (`Session Reference` :type "/Game/ExampleOSS/Common/BaseTasks/Session/BaseSessionReference Object Reference"))
  (bind (_sessionname _result) (`OnlineSessionSubsystemJoinSession.JoinSession` (subsystem `OnlineSessionSubsystem`) (`OnlineHelpers.GetControllerUniqueNetId` (`GameplayStatics.GetPlayerController` 0)) `Session Name` (`/Game/ExampleOSS/Blueprints/Session/BpSessionReference.Session` (cast `/Game/ExampleOSS/Blueprints/Session/BpSessionReference` `Session Reference` :!pure true)))
    (:`OnCallFailed`
      (`self.On Complete` false))
    (:`OnJoinSessionComplete`
      (`self.On Complete` (`|EnumEquality` _result "Success"))))
  (`self.K2_DestroyActor`))

(fn `UserConstructionScript`
  (`parent.UserConstructionScript`))