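; BpFindSessionsTask is a one-shot example task actor that searches the online subsystem for game sessions.
; FindSessions builds an OnlineSessionSearch with an attribute filter and limits, then runs it for the first player controller.
; Results are wrapped in BpSessionReference objects and passed to CallOnComplete, or an empty list on call failure, before the actor destroys itself.
; A Steam-specific PRESENCESEARCH branch exists but is unconnected.
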(event `self.Find Sessions`
  ;[0 0 0] Create the search object. This will hold the settings and then once the search finishes running, it will hold the search results.
  (bind _returnvalue (`|GenericCreateObject` (`GameplayStatics.GetPlayerController` 0) "/Script/OnlineSubsystemBlueprints.OnlineSessionSearch"))
  (set `self.Online Search` _returnvalue)
  ;[0 0 0] Here we configure the search we're about to run. We set the search parameters (which match against attributes), as well as other values. Not all subsystems use things like "Timeout in Seconds", so you can omit these extra settings in most cases. They are shown here for completeness.
  (`|ExecutionSequence`
    (:`then_0`
      (set `OnlineSessionSearch.SearchParams` (`|MakeMap` "SessionSetting" (make `SessionSearchParamBP` (make `VariantDataBP` "String" false 0 0.0 0 "SettingValue")) :!type "Name") (`self.Online Search`)))
    (:`then_1`
      (set `OnlineSessionSearch.bIsLanQuery` false (`self.Online Search`)))
    (:`then_2`
      (set `OnlineSessionSearch.PingBucketSize` 0 (`self.Online Search`)))
    (:`then_3`
      (set `OnlineSessionSearch.PlatformHash` 0 (`self.Online Search`)))
    (:`then_4`
      (set `OnlineSessionSearch.TimeoutInSeconds` 120.0 (`self.Online Search`)))
    (:`then_5`
      (set `OnlineSessionSearch.MaxSearchResults` 100 (`self.Online Search`)))
    (:`then_6`
      ;[0 0 0] Now run the search. Note that the For Each Loop after On Find Sessions Complete is just wrapping the result for the example. You can use the result objects directly (which are the search results that contain information about the sessions that were found).
      (bind _bwassuccessful (`OnlineSessionSubsystemFindSessions.FindSessions` (subsystem `OnlineSessionSubsystem`) (`OnlineHelpers.GetControllerUniqueNetId` (`GameplayStatics.GetPlayerController` 0)) (`self.Online Search`))
        (:`OnCallFailed`
          (`self.On Complete` false (`|MakeArray`))
          (`self.K2_DestroyActor`))
        (:`OnFindSessionsComplete`
          (set `self.Results` (`|MakeArray`))
          (for _array_element (`OnlineSessionSearch.GetSearchResults` (`self.Online Search`))
            (bind _returnvalue_2 (`|GenericCreateObject` (`GameplayStatics.GetPlayerController` 0) "/Game/ExampleOSS/Blueprints/Session/BpSessionReference.BpSessionReference_C" _array_element))
            (`KismetArrayLibrary.Array_Add` (`self.Results`) _returnvalue_2))
          (`self.On Complete` _bwassuccessful (`self.Results`))
          (`self.K2_DestroyActor`))))))

(fn `UserConstructionScript`
  (`parent.UserConstructionScript`))