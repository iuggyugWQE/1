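; A one-shot task actor that creates an advertised, joinable online session with a given name and capacity in an online subsystem example.
; It hosts under the first player controller's net ID, or creates a "DEDICATED_SERVER" ID when no controller exists.
; An async session call applies presence, invite and sample custom settings.
; Completion or call failure reports success or failure through CallOnComplete, then destroys the actor.
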(event `self.Create Session`
  (params (`Session Name` :type Name) (Capacity :type Integer))
  (bind _returnvalue (`GameplayStatics.GetPlayerController` 0))
  (if (`KismetSystemLibrary.IsValid` _returnvalue)
    (set `self.Hosting Player Id` (`OnlineHelpers.GetControllerUniqueNetId` _returnvalue))
    (else
      (bind _returnvalue_2 (`OnlineIdentitySubsystem.CreateUniquePlayerId` (subsystem `OnlineIdentitySubsystem`) "DEDICATED_SERVER"))
      (set `self.Hosting Player Id` _returnvalue_2)))
  (bind (_sessionname _bwassuccessful) (`OnlineSessionSubsystemCreateSession.CreateSession` (subsystem `OnlineSessionSubsystem`) (`self.Hosting Player Id`) `Session Name` (make `OnlineSessionSettingsBP` Capacity 0 true true false false false true true true false false 0 (`|MakeMap` "SessionSetting" (make `OnlineSessionSettingBP` (make `VariantDataBP` "String" false 0 0.0 0 "SettingValue") "ViaOnlineService") :!type "Name")))
    (:`OnCallFailed`
      (`self.On Complete` false))
    (:`OnCreateSessionComplete`
      (`self.On Complete` _bwassuccessful)))
  (`self.K2_DestroyActor`))

(fn `UserConstructionScript`
  (`parent.UserConstructionScript`))