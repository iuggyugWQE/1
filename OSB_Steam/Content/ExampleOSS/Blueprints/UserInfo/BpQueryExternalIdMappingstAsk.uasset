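; One-shot task actor in the OSS example that looks up which users are linked to external account IDs on a given platform.
; It splits the input string into IDs and runs an async OnlineUserSubsystem query as the first player controller's user.
; On success it reads each mapping from the subsystem cache and reports joined "external->user" pairs through CallOnComplete.
; Failures report an error message, and every outcome destroys the actor.
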(event `self.Query External Id Mappings`
  (params (`Platform Type` :type String) (`External Ids` :type String))
  (bind _externalidqueryoptionsbp (make `ExternalIdQueryOptionsBP` false `Platform Type`))
  ;[0 0 0] Query the external ID mappings and discover the user associated with it (if any). The result is stored in the cache.
  (bind (_bwassuccessful _userid _queryoptions _externalids _error) (`OnlineUserSubsystemQueryExternalIdMappings.QueryExternalIdMappings` (subsystem `OnlineUserSubsystem`) (`OnlineHelpers.GetControllerUniqueNetId` (`GameplayStatics.GetPlayerController` 0)) _externalidqueryoptionsbp (`KismetStringLibrary.ParseIntoArray` `External Ids` " \n"))
    (:`OnCallFailed`
      (`self.On Complete` "Failed to query external ID mappings.")
      (`self.K2_DestroyActor` :!label _label))
    (:`OnQueryExternalIdMappingsComplete`
      (if _bwassuccessful
        ;[0 0 0] Get the retrieved information from the cache and return the mapping of external ID to user ID.
        (set `self.Found User IDs` (`|MakeArray`))
        (for _array_element _externalids
          (bind _returnvalue (`OnlineUserSubsystem.GetExternalIdMapping` (subsystem `OnlineUserSubsystem`) _externalidqueryoptionsbp _array_element))
          (`KismetArrayLibrary.Array_Add` (`self.Found User IDs`) (`KismetStringLibrary.Concat_StrStr` _array_element " -> " (`OnlineHelpers.Conv_FUniqueNetIdReplToString` _returnvalue))))
        (`self.On Complete` (`KismetStringLibrary.JoinStringArray` (`self.Found User IDs`) " \n"))
        (`self.K2_DestroyActor`)
        (else
          (`self.On Complete` (`KismetStringLibrary.Concat_StrStr` "Failed to query: " _error))
          (goto _label))))))

(fn `UserConstructionScript`
  (`parent.UserConstructionScript`))