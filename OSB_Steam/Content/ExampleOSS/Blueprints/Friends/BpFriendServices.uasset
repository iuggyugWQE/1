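; Friends service Blueprint for the ExampleOSS project, wrapping the online friends subsystem for the first local user.
; On BeginPlay it binds to the subsystem's friends-change event and relays it through an OnFriendsListChanged dispatcher.
; GetCachedFriends wraps each entry of the already-loaded list in a BpFriendReference object, without starting a fetch.
; IsFriend and IsBlockedPlayer linearly search the friends and blocked lists, comparing user IDs as strings.
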(event `self.ReceiveBeginPlay`
  (add `OnlineFriendsSubsystem.OnFriendsChange` (subsystem `OnlineFriendsSubsystem`) (delegate `Handle Friends Change`)))

(event `Handle Friends Change`
  (params (LocalUserNum :type Integer))
  (`self.On Friends List Changed`))

(fn `Get Cached Friends`
  (returns (Friends :type "Array of /Game/ExampleOSS/Common/BaseTasks/Friends/BaseFriendReference Object Reference"))
  (locals (Results :type "Array of /Game/ExampleOSS/Common/BaseTasks/Friends/BaseFriendReference Object Reference"))
  (bind (_outfriends _returnvalue) (`OnlineFriendsSubsystem.GetFriendsList` (subsystem `OnlineFriendsSubsystem`) 0 ""))
  (if _returnvalue
    (set `local.Results` (`|MakeArray`))
    (for _array_element _outfriends
      (bind _returnvalue_2 (`|GenericCreateObject` (`GameplayStatics.GetPlayerController` 0) "/Game/ExampleOSS/Blueprints/Friends/BpFriendReference.BpFriendReference_C" _array_element))
      (`KismetArrayLibrary.Array_Add` (`local.Results`) _returnvalue_2))
    (return (`local.Results`))))

(fn `Is Blocked Player`
  (params (`User ID` :type String))
  (returns (Result :type Boolean))
  (bind _outblockedplayers (`OnlineFriendsSubsystem.GetBlockedPlayers` (subsystem `OnlineFriendsSubsystem`) (`OnlineIdentitySubsystem.GetUniquePlayerId` (subsystem `OnlineIdentitySubsystem`) 0)))
  (for _array_element _outblockedplayers
    (if (`KismetStringLibrary.EqualEqual_StrStr` `User ID` (`OnlineHelpers.Conv_FUniqueNetIdReplToString` (`OnlineUserRef.GetUserId` _array_element)))
      (return true)))
  (return false))

(fn `Is Friend`
  (params (`User ID` :type String))
  (returns (Result :type Boolean))
  (bind _outfriends (`OnlineFriendsSubsystem.GetFriendsList` (subsystem `OnlineFriendsSubsystem`) 0 ""))
  (for _array_element _outfriends
    (if (`KismetStringLibrary.EqualEqual_StrStr` `User ID` (`OnlineHelpers.Conv_FUniqueNetIdReplToString` (`OnlineUserRef.GetUserId` _array_element)))
      (return true)))
  (return false))

(fn `UserConstructionScript`
  (`parent.UserConstructionScript`))