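; Task actor in the Example OSS project that removes the local player from an online party.
; The LeaveParty event reads the party ID from a BpPartyIdReference and calls the online party subsystem's async LeaveParty for the first player controller's unique net ID.
; It reports completion as successful only on a Succeeded result, reports failure if the call fails, then destroys itself.
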(event `self.Leave Party`
  (params (`Party Id` :type "/Game/ExampleOSS/Common/BaseTasks/Parties/BasePartyIdReference Object Reference"))
  (bind (_localuserid _partyid _result) (`OnlinePartySubsystemLeaveParty.LeaveParty` (subsystem `OnlinePartySubsystem`) (`OnlineHelpers.GetControllerUniqueNetId` (`GameplayStatics.GetPlayerController` 0)) (`/Game/ExampleOSS/Blueprints/Parties/BpPartyIdReference.Party Id` (cast `/Game/ExampleOSS/Blueprints/Parties/BpPartyIdReference` `Party Id` :!pure true)))
    (:`OnCallFailed`
      (`self.On Complete` false))
    (:`OnLeavePartyComplete`
      (`self.On Complete` (`|EnumEquality` _result "Succeeded"))))
  (`self.K2_DestroyActor`))

(fn `UserConstructionScript`
  (`parent.UserConstructionScript`))