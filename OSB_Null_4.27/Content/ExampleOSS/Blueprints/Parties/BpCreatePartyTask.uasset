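; BpCreatePartyTask is a short-lived actor that creates an online party for the first local player through the Online Party Subsystem.
; CreateParty requests a primary-type party with auto-approved joins, open presence and invites, chat and a small member cap.
; It reports success or failure through CallOnComplete on either async outcome, then destroys itself.
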(event `self.Create Party`
  (bind (_localuserid _partyid _result) (`OnlinePartySubsystemCreateParty.CreateParty` (subsystem `OnlinePartySubsystem`) (`OnlineHelpers.GetControllerUniqueNetId` (`GameplayStatics.GetPlayerController` 0)) (`OnlineHelpers.GetPrimaryPartyType`) (make `OnlinePartyConfiguration` "AutoApprove" "Anyone" "Anyone" true false true 0 4))
    (:`OnCallFailed`
      (`self.On Complete` false))
    (:`OnCreatePartyComplete`
      (`self.On Complete` (`|EnumEquality` _result "Succeeded"))))
  (`self.K2_DestroyActor`))

(fn `UserConstructionScript`
  (`parent.UserConstructionScript`))