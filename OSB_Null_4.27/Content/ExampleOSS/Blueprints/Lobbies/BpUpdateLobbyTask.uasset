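; A short-lived task actor that updates an online lobby through the lobby subsystem, in the Online Subsystem example content.
; UpdateLobby builds an update transaction for the first player controller's user ID, writing the given value to the "TestInteger" Int64 metadata key.
; It runs the async lobby update, reports success or failure with the lobby ID through the OnComplete dispatcher, then destroys itself.
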(event `self.Update Lobby`
  (params (`Lobby Id` :type "/Game/ExampleOSS/Common/BaseTasks/Lobbies/BaseLobbyIdRef Object Reference") (`Test Attribute Value` :type Integer64) (`Lobby Services` :type "/Game/ExampleOSS/Common/BaseTasks/Lobbies/BaseLobbyServices Object Reference"))
  (bind _returnvalue (subsystem `OnlineLobbySubsystem`))
  (bind _lobby_id (`/Game/ExampleOSS/Blueprints/Lobbies/BpLobbyIdRef.Lobby Id` (cast `/Game/ExampleOSS/Blueprints/Lobbies/BpLobbyIdRef` `Lobby Id` :!pure true)))
  (bind _returnvalue_2 (`OnlineLobbySubsystem.MakeUpdateLobbyTransaction` _returnvalue (`OnlineHelpers.GetControllerUniqueNetId` (`GameplayStatics.GetPlayerController` 0)) _lobby_id))
  (`OnlineLobbyTransaction.SetMetadata` _returnvalue_2 "TestInteger" (make `VariantDataBP` "Int64" false 0 0.0 `Test Attribute Value`))
  (bind _error (`OnlineLobbySubsystemUpdateLobby.UpdateLobby` _returnvalue (`OnlineHelpers.GetControllerUniqueNetId` (`GameplayStatics.GetPlayerController` 0)) _lobby_id _returnvalue_2)
    (:`OnCallFailed`
      (`self.On Complete` false `Lobby Id` :!label _label))
    (:`OnLobbyOperationComplete`
      (if (break `OnlineErrorInfo` _error)
        (`self.On Complete` true `Lobby Id`)
        (else
          (goto _label)))))
  (`self.K2_DestroyActor`))

(fn `UserConstructionScript`
  (`parent.UserConstructionScript`))