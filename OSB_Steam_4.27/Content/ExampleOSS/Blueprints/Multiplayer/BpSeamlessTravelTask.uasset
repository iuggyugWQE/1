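; Multiplayer example Blueprint that performs seamless server travel between two test maps, MultiplayerMap and MultiplayerMap2.
; Its SeamlessTravel event enables seamless travel on the game mode, then reads the current map name from the first MapNameActor in the level.
; It picks the opposite map from that name and issues a servertravel console command through player controller 0.
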(event `self.Seamless Travel`
  (set `GameModeBase.bUseSeamlessTravel` true (`GameplayStatics.GetGameMode`))
  (bind _outactors (`GameplayStatics.GetAllActorsOfClass` "/Game/ExampleOSS/Common/Multiplayer/MapNameActor.MapNameActor_C"))
  (`KismetSystemLibrary.ExecuteConsoleCommand` (`KismetStringLibrary.Concat_StrStr` "servertravel " (`KismetMathLibrary.SelectString` "/Game/ExampleOSS/Common/Multiplayer/MultiplayerMap2" "/Game/ExampleOSS/Common/Multiplayer/MultiplayerMap" (`KismetStringLibrary.EqualEqual_StrStr` (`/Game/ExampleOSS/Common/Multiplayer/MapNameActor.Map Name` (`|GetArrayItem` _outactors)) "MultiplayerMap"))) (`GameplayStatics.GetPlayerController` 0)))

(fn `UserConstructionScript`
  (`parent.UserConstructionScript`))