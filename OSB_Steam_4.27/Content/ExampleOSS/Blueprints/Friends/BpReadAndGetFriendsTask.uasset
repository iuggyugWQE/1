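; An example task actor that reads the local user's friends list from the online friends subsystem and returns it as BpFriendReference objects.
; An async read is followed by a get, with each friend wrapped in a reference object after an injected emulated friend that demonstrates deriving OSB types.
; It reports success with the results, or failure with an empty list, through CallOnComplete, then destroys itself.
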(event `self.Read and Get Friends`
  (bind (_localusernum _bwassuccessful) (`OnlineFriendsSubsystemReadFriendsList.ReadFriendsList` (subsystem `OnlineFriendsSubsystem`))
    (:`OnCallFailed`
      (`self.On Complete` false (`|MakeArray`) :!label _label)
      (`self.K2_DestroyActor`))
    (:`OnReadFriendsListComplete`
      (if _bwassuccessful
        (bind (_outfriends _returnvalue) (`OnlineFriendsSubsystem.GetFriendsList` (subsystem `OnlineFriendsSubsystem`) 0 ""))
        (if _returnvalue
          (bind _output_get (set `self.Results` (`|MakeArray`)))
          ;[1 1 1] Add emulated friend (example on how to derive OSB types for your own usage)
          (bind _returnvalue_2 (`|GenericCreateObject` "/Game/ExampleOSS/Blueprints/Friends/EmulatedFriendRef.EmulatedFriendRef_C" self))
          (bind _returnvalue_3 (`|GenericCreateObject` "/Game/ExampleOSS/Blueprints/Friends/BpFriendReference.BpFriendReference_C" self _returnvalue_2))
          (`KismetArrayLibrary.Array_Add` _output_get _returnvalue_3)
          ;[1 1 1] Add the actual friends
          (for _array_element _outfriends
            (bind _returnvalue_4 (`|GenericCreateObject` "/Game/ExampleOSS/Blueprints/Friends/BpFriendReference.BpFriendReference_C" self _array_element))
            (`KismetArrayLibrary.Array_Add` (`self.Results`) _returnvalue_4))
          (`self.On Complete` true (`self.Results`))
          (`self.K2_DestroyActor`)
          (else
            (goto _label)))
        (else
          (goto _label))))))

(fn `UserConstructionScript`
  (`parent.UserConstructionScript`))