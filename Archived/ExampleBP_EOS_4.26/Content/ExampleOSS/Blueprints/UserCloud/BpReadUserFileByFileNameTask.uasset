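; A one-shot task actor that reads a named file from the online user cloud for the first player controller's user.
; It runs the async ReadUserFile call, then fetches the file contents from the subsystem and converts them to a string.
; It reports success with that string, or failure with an empty one, through OnComplete and then destroys itself.
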(event `self.Read User File`
  (params (Filename :type String))
  (bind _returnvalue (subsystem `OnlineUserCloudSubsystem`))
  (bind (_bwassuccessful _userid _filename) (`OnlineUserCloudSubsystemReadUserFile.ReadUserFile` _returnvalue (`OnlineHelpers.GetControllerUniqueNetId` (`GameplayStatics.GetPlayerController` 0)) Filename)
    (:`OnCallFailed`
      (`self.On Complete` false :!label _label))
    (:`OnReadUserFileComplete`
      (if _bwassuccessful
        (bind (_filecontents _returnvalue_2) (`OnlineUserCloudSubsystem.GetFileContents` _returnvalue _userid _filename))
        (if _returnvalue_2
          (bind _returnvalue_3 (`OnlineHelpers.ReadFileDataAsString` _filecontents))
          (`self.On Complete` true _returnvalue_3)
          (else
            (goto _label)))
        (else
          (goto _label)))))
  (`self.K2_DestroyActor`))

(fn `UserConstructionScript`
  (`parent.UserConstructionScript`))