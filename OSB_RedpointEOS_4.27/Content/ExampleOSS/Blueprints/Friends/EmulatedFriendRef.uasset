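; Example subclass of UOnlineFriendRef that emulates a friend from a non-OSB system, so it can share one friend list with OSB friends.
; It overrides the friend getters with hardcoded data: an accepted invite, online in-game presence, an explanatory display name and a placeholder real name.
; The user ID is a default-constructed net ID, and attribute lookups and writes always report failure.
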(fn `GetDisplayName`
  (returns (ReturnValue :type String))
  (return "This is an example on how to derive UOnlineFriendRef to emulate friend objects from your own systems (instead of OSB), and still be able to store all friends (your system + OSB) in a single list. Refer to EmulatedFriendRef and BpReadAndGetFriendsTask to see how this is set up."))

(fn `GetInviteStatus`
  (returns (ReturnValue :type "EInviteStatus_ Enum"))
  (return "Accepted"))

(fn `GetPresence`
  (returns (ReturnValue :type "OnlineUserPresenceData Structure"))
  (return (make `OnlineUserPresenceData` "INVALID" true true true false false "0001.01.01-00.00.00" (make `OnlineUserPresenceStatusData` "Emulated"))))

(fn `GetRealName`
  (returns (ReturnValue :type String))
  (return "Emulated Real Name"))

(fn `GetUserAttribute`
  (params (Key :type String))
  (returns (Found :type Boolean) (ReturnValue :type String))
  (return false ""))

(fn `GetUserId`
  (returns (ReturnValue :type "UniqueNetIdRepl Structure"))
  (return (make `UniqueNetIdRepl`)))

(fn `SetUserLocalAttribute`
  (params (Key :type String) (Value :type String))
  (returns (Success :type Boolean))
  (return false))