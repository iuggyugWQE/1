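; Example lobby service that wraps the online lobby and party subsystems behind reference objects for lobby IDs, members and party invites.
; It lists lobbies from its JoinedLobbies array and prunes that array in reverse when the subsystem reports a lobby deleted.
; Member queries use the first local player's net ID to gather user IDs by index.
; A helper converts lobby IDs into party join info, logging on failure.
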(event `self.ReceiveBeginPlay`
  (add `OnlineLobbySubsystem.OnLobbyDelete` (subsystem `OnlineLobbySubsystem`) (delegate `On Lobby Delete`)))

(event `On Lobby Delete`
  (params (UserId :type "UniqueNetIdRepl Structure") (LobbyId :type "LobbyId Object Reference"))
  (bind _returnvalue (`|GenericCreateObject` "/Game/ExampleOSS/Blueprints/Lobbies/BpLobbyIdRef.BpLobbyIdRef_C" self LobbyId))
  (`self.Remove Joined Lobby` _returnvalue))

(fn `Convert Lobby Id to Party Join Info`
  (params (`Lobby Id` :type "/Game/ExampleOSS/Common/BaseTasks/Lobbies/BaseLobbyIdRef Object Reference"))
  (returns (`Party Invite` :type "/Game/ExampleOSS/Common/BaseTasks/Parties/BasePartyInviteReference Object Reference"))
  (bind _returnvalue (`OnlineHelpers.Conv_ULobbyIdToUOnlinePartyJoinInfo` (`OnlineHelpers.GetControllerUniqueNetId` (`GameplayStatics.GetPlayerController` 0)) (subsystem `OnlinePartySubsystem`) (`/Game/ExampleOSS/Blueprints/Lobbies/BpLobbyIdRef.Lobby Id` (cast `/Game/ExampleOSS/Blueprints/Lobbies/BpLobbyIdRef` `Lobby Id` :!pure true))))
  (`/Engine/EditorBlueprintResources/StandardMacros.IsValid` _returnvalue
    (:`Is Valid`
      (bind _returnvalue_2 (`|GenericCreateObject` "/Game/ExampleOSS/Blueprints/Parties/BpPartyInviteReference.BpPartyInviteReference_C" self _returnvalue))
      (return _returnvalue_2))
    (:`Is Not Valid`
      (`KismetSystemLibrary.PrintString` "Unable to convert lobby ID to party join info!" false true (struct :`R` 1.0 :`A` 1.0))
      (return null))))

(fn `Get Joined Lobbies`
  (returns (Lobbies :type "Array of /Game/ExampleOSS/Common/BaseTasks/Lobbies/BaseLobbyIdRef Object Reference"))
  (locals (`Lobby Ids` :type "Array of /Game/ExampleOSS/Common/BaseTasks/Lobbies/BaseLobbyIdRef Object Reference"))
  (for _array_element (`self.Joined Lobbies`)
    (bind _returnvalue (`|GenericCreateObject` "/Game/ExampleOSS/Blueprints/Lobbies/BpLobbyIdRef.BpLobbyIdRef_C" self (`Lobby.GetId` (`/Game/ExampleOSS/Blueprints/Lobbies/BpLobbyRef.Lobby` _array_element))))
    (`KismetArrayLibrary.Array_Add` (`local.Lobby Ids`) _returnvalue))
  (return (`local.Lobby Ids`)))

(fn `Get Lobby Members`
  (params (`Lobby Id` :type "/Game/ExampleOSS/Common/BaseTasks/Lobbies/BaseLobbyIdRef Object Reference"))
  (returns (Members :type "Array of /Game/ExampleOSS/Common/BaseTasks/Lobbies/BaseLobbyMemberIdRef Object Reference"))
  (locals (`Lobby Members` :type "Array of /Game/ExampleOSS/Common/BaseTasks/Lobbies/BaseLobbyMemberIdRef Object Reference"))
  (bind _lobby_id (`/Game/ExampleOSS/Blueprints/Lobbies/BpLobbyIdRef.Lobby Id` (cast `/Game/ExampleOSS/Blueprints/Lobbies/BpLobbyIdRef` `Lobby Id` :!pure true)))
  (bind (_outmembercount _returnvalue) (`OnlineLobbySubsystem.GetMemberCount` (subsystem `OnlineLobbySubsystem`) (`OnlineHelpers.GetControllerUniqueNetId` (`GameplayStatics.GetPlayerController` 0)) _lobby_id))
  (if _returnvalue
    (for _index (range _outmembercount)
      (bind (_outmemberid _returnvalue_2) (`OnlineLobbySubsystem.GetMemberUserId` (subsystem `OnlineLobbySubsystem`) (`OnlineHelpers.GetControllerUniqueNetId` (`GameplayStatics.GetPlayerController` 0)) _lobby_id _index))
      (if _returnvalue_2
        (bind _returnvalue_3 (`|GenericCreateObject` "/Game/ExampleOSS/Blueprints/Lobbies/BpLobbyMemberIdRef.BpLobbyMemberIdRef_C" self _outmemberid))
        (`KismetArrayLibrary.Array_Add` (`local.Lobby Members`) _returnvalue_3)))
    (return (`local.Lobby Members`))
    (else
      (return (`|MakeArray`)))))

(fn `Remove Joined Lobby`
  (params (`Lobby Id` :type "/Game/ExampleOSS/Blueprints/Lobbies/BpLobbyIdRef Object Reference"))
  (locals (Max :type Integer))
  (bind _output_get (set `local.Max` (- (`KismetArrayLibrary.Array_Length` (`self.Joined Lobbies`)) 1)))
  (for _index (range (+ _output_get 1))
    (bind _returnvalue (- (`local.Max`) _index))
    (if (== (`Lobby.GetId` (`/Game/ExampleOSS/Blueprints/Lobbies/BpLobbyRef.Lobby` (`|GetArrayItem` (`self.Joined Lobbies`) _returnvalue))) (`/Game/ExampleOSS/Blueprints/Lobbies/BpLobbyIdRef.Lobby Id` `Lobby Id`))
      (`KismetArrayLibrary.Array_Remove` (`self.Joined Lobbies`) _returnvalue))))

(fn `UserConstructionScript`
  (`parent.UserConstructionScript`))