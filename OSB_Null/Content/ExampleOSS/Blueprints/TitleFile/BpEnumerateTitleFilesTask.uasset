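; Async task actor that lists the title files available from the online subsystem for the OSS example.
; EnumerateTitleFilenames calls EnumerateFiles on the title file subsystem with an unbounded paged query.
; On success it wraps each GetFileList entry in a BpFileEntry object and passes the array to OnComplete.
; Failures report OnComplete with false and an empty list, and the actor destroys itself afterward in either case.
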(event `self.Enumerate Title Filenames`
  (bind _bwassuccessful (`OnlineTitleFileSubsystemEnumerateFiles.EnumerateFiles` (subsystem `OnlineTitleFileSubsystem`) (make `PagedQueryBP` 0 -1))
    (:`OnCallFailed`
      (`self.On Complete` false (`|MakeArray`) :!label _label)
      (`self.K2_DestroyActor`))
    (:`OnEnumerateFilesComplete`
      (if _bwassuccessful
        (bind _files (`OnlineTitleFileSubsystem.GetFileList` (subsystem `OnlineTitleFileSubsystem`)))
        (set `self.Files` (`|MakeArray`))
        (for _array_element _files
          (bind _returnvalue (`|GenericCreateObject` (`GameplayStatics.GetPlayerController` 0) "/Game/ExampleOSS/Blueprints/UserCloud/BpFileEntry.BpFileEntry_C" _array_element))
          (`KismetArrayLibrary.Array_Add` (`self.Files`) _returnvalue))
        (`self.On Complete` true (`self.Files`))
        (`self.K2_DestroyActor`)
        (else
          (goto _label))))))

(fn `UserConstructionScript`
  (`parent.UserConstructionScript`))