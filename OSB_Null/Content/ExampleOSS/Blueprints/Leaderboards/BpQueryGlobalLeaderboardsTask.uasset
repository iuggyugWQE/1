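; Task actor that queries a global online leaderboard by ID and returns its entries, then destroys itself.
; It reads a range of rows around a rank through the online leaderboards subsystem and converts them into entry structs of rank, player ID, nickname and score.
; Score always comes from the "Score" column, as EOS ranked searches require.
; A failed call or read completes unsuccessfully with an empty list.
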(event `self.Query Global Leaderboards`
  (params (`Leaderboard Id` :type String))
  (bind _array (`|MakeArray`))
  (bind _returnvalue (`|GenericCreateObject` "/Script/OnlineSubsystemBlueprints.OnlineLeaderboardRead" self))
  (`OnlineLeaderboardRead.SetLeaderboardName` _returnvalue (`KismetStringLibrary.Conv_StringToName` `Leaderboard Id`))
  (bind _bwassuccessful (`OnlineLeaderboardsSubsystemReadLeaderboardsAroundRank.ReadLeaderboardsAroundRank` (subsystem `OnlineLeaderboardsSubsystem`) 0 100 _returnvalue)
    (:`OnCallFailed`
      (`self.On Complete` false _array :!label _label)
      (`self.K2_DestroyActor`))
    (:`OnLeaderboardReadComplete`
      (if _bwassuccessful
        (set `self.Results` _array)
        (for _array_element (`OnlineLeaderboardRead.GetRows` _returnvalue)
          (`KismetArrayLibrary.Array_Add` (`self.Results`) (make `/Game/ExampleOSS/Common/BaseTasks/Leaderboards/LeaderboardEntryData` (`.Rank` (break `OnlineStatsRowBP` _array_element)) (`OnlineHelpers.Conv_FUniqueNetIdReplToString` (`.PlayerId` (break `OnlineStatsRowBP` _array_element))) (break `OnlineStatsRowBP` _array_element) (`.AsInt` (break `VariantDataBP` (`BlueprintMapLibrary.Map_Find` (`.Columns` (break `OnlineStatsRowBP` _array_element)) "Score"))))))
        (`self.On Complete` true (`self.Results`))
        (`self.K2_DestroyActor`)
        (else
          (goto _label))))))

(fn `UserConstructionScript`
  (`parent.UserConstructionScript`))