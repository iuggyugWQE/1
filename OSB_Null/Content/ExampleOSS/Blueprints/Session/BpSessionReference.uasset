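; BpSessionReference wraps an online session struct and exposes read-only queries on it for the ExampleOSS online subsystem example.
; It returns the session ID, plus open and total public connection slots.
; The dedicated server check looks up the IsDedicatedServer key in the session settings map and is true only when the key exists and its boolean value is true.
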(fn `Get Capacity`
  (returns (`Open Slots` :type Integer) (`Total Slots` :type Integer))
  (bind _session (`self.Session`))
  (return (`.NumOpenPublicConnections` (break `OnlineSessionBP` (break `OnlineSessionSearchResultBP` _session))) (`.NumPublicConnections` (break `OnlineSessionSettingsBP` (`.SessionSettings` (break `OnlineSessionBP` (break `OnlineSessionSearchResultBP` _session)))))))

(fn `Get Session Id`
  (returns (`Session Id` :type String))
  (return (`.SessionId` (break `OnlineSessionBP` (break `OnlineSessionSearchResultBP` (`self.Session`))))))

(fn `Is Dedicated Server?`
  (returns (`Dedicated Server` :type Boolean))
  (bind (_value _returnvalue) (`BlueprintMapLibrary.Map_Find` (`.Settings` (break `OnlineSessionSettingsBP` (`.SessionSettings` (break `OnlineSessionBP` (break `OnlineSessionSearchResultBP` (`self.Session`)))))) "IsDedicatedServer"))
  (return (and (`.AsBool` (break `VariantDataBP` (break `OnlineSessionSettingBP` _value))) _returnvalue)))