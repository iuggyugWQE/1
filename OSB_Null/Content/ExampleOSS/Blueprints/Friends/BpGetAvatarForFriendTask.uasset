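; Short-lived actor task that fetches an online avatar texture for one friend in the ExampleOSS friends example.
; FetchFriendAvatar casts the friend to BpFriendReference and runs the async GetAvatar call on the Online Avatar Subsystem for the first local player.
; It passes the result to CallOnAvatarFetched, using a FontAwesome user icon on failure, then destroys itself.
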(event `self.Fetch Friend Avatar`
  (params (Friend :type "/Game/ExampleOSS/Common/BaseTasks/Friends/BaseFriendReference Object Reference"))
  (bind _returnvalue (`OnlineUserRef.GetUserId` (`/Game/ExampleOSS/Blueprints/Friends/BpFriendReference.Friend` (cast `/Game/ExampleOSS/Blueprints/Friends/BpFriendReference` Friend :!pure true))))
  (`KismetSystemLibrary.PrintString` (`KismetStringLibrary.Concat_StrStr` "Blueprint fetching avatar for: " (`OnlineHelpers.Conv_FUniqueNetIdReplToString` _returnvalue)))
  (bind (_bwassuccessful _resulttexture) (`OnlineAvatarSubsystemGetAvatar.GetAvatar` (subsystem `OnlineAvatarSubsystem`) (`OnlineHelpers.GetControllerUniqueNetId` (`GameplayStatics.GetPlayerController` 0)) _returnvalue "/Game/ExampleOSS/Common/UIComponents/FontAwesomeUserIcon.FontAwesomeUserIcon")
    (:`OnCallFailed`
      (`self.On Avatar Fetched` Friend "/Game/ExampleOSS/Common/UIComponents/FontAwesomeUserIcon.FontAwesomeUserIcon"))
    (:`OnGetAvatarComplete`
      (`self.On Avatar Fetched` Friend _resulttexture)))
  (`self.K2_DestroyActor`))

(fn `UserConstructionScript`
  (`parent.UserConstructionScript`))