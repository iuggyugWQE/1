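; One-shot task actor that fetches the local player's recent players list from the online friends subsystem.
; ReadRecentPlayers runs an async query for player 0, then reads the result and wraps each entry in a BpSimpleUserReference holding ID string and display name.
; It passes that array, or an empty one if the call fails, to OnComplete, then destroys itself.
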(event `self.Read Recent Players`
  (bind _returnvalue (subsystem `OnlineFriendsSubsystem`))
  (bind (_userid _namespace) (`OnlineFriendsSubsystemQueryRecentPlayers.QueryRecentPlayers` _returnvalue (`OnlineIdentitySubsystem.GetUniquePlayerId` (subsystem `OnlineIdentitySubsystem`) 0))
    (:`OnCallFailed`
      (`self.On Complete` (`|MakeArray`))
      (`self.K2_DestroyActor`))
    (:`OnQueryRecentPlayersComplete`
      (bind _outrecentplayers (`OnlineFriendsSubsystem.GetRecentPlayers` _returnvalue _userid _namespace))
      (set `self.Results` (`|MakeArray`))
      (for _array_element _outrecentplayers
        (bind _returnvalue_2 (`|GenericCreateObject` (`GameplayStatics.GetPlayerController` 0) "/Game/ExampleOSS/Blueprints/Friends/BpSimpleUserReference.BpSimpleUserReference_C" (`OnlineHelpers.Conv_FUniqueNetIdReplToString` (`OnlineUserRef.GetUserId` _array_element)) (`OnlineUserRef.GetDisplayName` _array_element)))
        (`KismetArrayLibrary.Array_Add` (`self.Results`) _returnvalue_2))
      (`self.On Complete` (`self.Results`))
      (`self.K2_DestroyActor`))))

(fn `UserConstructionScript`
  (`parent.UserConstructionScript`))