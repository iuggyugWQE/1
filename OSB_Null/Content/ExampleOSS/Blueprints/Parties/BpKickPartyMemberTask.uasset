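; BpKickPartyMemberTask is an example online subsystem task actor that kicks a member from a party.
; KickMember unwraps the party and member ID reference objects, then makes an async KickMember call on the party subsystem as the first local player.
; It reports success only when the result is Succeeded, reports failure if the call fails, and destroys itself afterward in both cases.
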(event `self.Kick Member`
  (params (`Party Id` :type "/Game/ExampleOSS/Common/BaseTasks/Parties/BasePartyIdReference Object Reference") (`Party Member Id` :type "/Game/ExampleOSS/Common/BaseTasks/Parties/BasePartyMemberIdReference Object Reference"))
  (bind (_localuserid _partyid _memberid _result) (`OnlinePartySubsystemKickMember.KickMember` (subsystem `OnlinePartySubsystem`) (`OnlineHelpers.GetControllerUniqueNetId` (`GameplayStatics.GetPlayerController` 0)) (`/Game/ExampleOSS/Blueprints/Parties/BpPartyIdReference.Party Id` (cast `/Game/ExampleOSS/Blueprints/Parties/BpPartyIdReference` `Party Id` :!pure true)) (`BlueprintPartyMember.GetUserId` (`/Game/ExampleOSS/Blueprints/Parties/BpPartyMemberIdReference.Party Member` (cast `/Game/ExampleOSS/Blueprints/Parties/BpPartyMemberIdReference` `Party Member Id` :!pure true))))
    (:`OnCallFailed`
      (`self.On Complete` false))
    (:`OnKickPartyMemberComplete`
      (`self.On Complete` (`|EnumEquality` _result "Succeeded"))))
  (`self.K2_DestroyActor`))

(fn `UserConstructionScript`
  (`parent.UserConstructionScript`))