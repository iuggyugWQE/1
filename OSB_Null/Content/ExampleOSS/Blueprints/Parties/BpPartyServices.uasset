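; Example party service Blueprint wrapping the online party subsystem for the local player.
; Query functions wrap joined parties, members and invites in reference objects and check leader and kick permissions.
; Invite events trigger a change notification, while party data updates let non-leaders follow their leader into a session.
; The "SessionFollowString" attribute carries a de-duplication ID and session ID, used to find and join the session before notifying the connection code.
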(event `self.ReceiveBeginPlay`
  (bind _returnvalue (subsystem `OnlinePartySubsystem`))
  (add `OnlinePartySubsystem.OnPartyInviteReceived` _returnvalue (delegate `On Party Invite Received`))
  (add `OnlinePartySubsystem.OnPartyDataReceived` _returnvalue (delegate `On Party Data Updated`)))

(event `On Party Invite Received`
  (params (LocalUserId :type "UniqueNetIdRepl Structure") (PartyId :type "PartyId Object Reference") (SenderId :type "UniqueNetIdRepl Structure"))
  (`self.On Invites Changed`))

(event `On Party Data Updated`
  (params (LocalUserId :type "UniqueNetIdRepl Structure") (PartyId :type "PartyId Object Reference") (Namespace :type Name) (PartyData :type "ReadablePartyData Object Reference"))
  (bind (_outfound _outattrvalue) (`ReadablePartyData.GetAttribute` PartyData "SessionFollowString"))
  (bind (_type _asbool _asint _asfloat _asint64 _asstring) (break `VariantDataBP` _outattrvalue))
  (bind (_lefts _rights) (`KismetStringLibrary.Split` _asstring "|"))
  ;[0 0 0] Check if we are the party leader. If we're the party leader, then we don't care about the party data being updated.
  ;
  ; The only reason party data will be updated in this example is if the party leader is setting a session follow string, and if we've done that as the leader, then we've already joined the session anyway, so we don't need to handle it here.
  (bind _returnvalue (`Party.GetLeaderId` (`OnlinePartySubsystem.GetParty` (subsystem `OnlinePartySubsystem`) LocalUserId PartyId)))
  (if (not (== _returnvalue LocalUserId))
    ;[0 0 0] If the SessionFollowString attribute is set and it's a string...
    (if _outfound
      (if (`|EnumEquality` _type "String")
        ;[0 0 0] If we've already handled this session follow before, ignore it.
        (if (not (`BlueprintSetLibrary.Set_Contains` (`self.Session Follow Consumed Ids`) _lefts))
          ;[0 0 0] Search for the session that the leader joined, so that we can join it.
          (`BlueprintSetLibrary.Set_Add` (`self.Session Follow Consumed Ids`) _lefts)
          (bind _returnvalue_2 (`OnlineSessionSubsystem.CreateSessionIdFromString` (subsystem `OnlineSessionSubsystem`) _rights))
          (bind (_localusernum _bwassuccessful _searchresult) (`OnlineSessionSubsystemFindSessionById.FindSessionById` (subsystem `OnlineSessionSubsystem`) (`OnlineHelpers.GetControllerUniqueNetId` (`GameplayStatics.GetPlayerController` 0)) _returnvalue_2)
            (:`then`
              ;[0 0 0] Join the session that we found.
              (bind (_sessionname _result) (`OnlineSessionSubsystemJoinSession.JoinSession` (subsystem `OnlineSessionSubsystem`) (`OnlineHelpers.GetControllerUniqueNetId` (`GameplayStatics.GetPlayerController` 0)) (`KismetStringLibrary.Conv_StringToName` _rights) _searchresult)
                (:`OnCallFailed`
                  (`KismetSystemLibrary.PrintString` "Unable to join session indicated by session follow request." :!label _label))
                (:`OnJoinSessionComplete`
                  (if (`|EnumEquality` _result "Success")
                    ;[0 0 0] Propagate back out to the example code which handles connecting to the server
                    (`self.On Party Leader Was Followed to Session` _sessionname)
                    (else
                      (goto _label))))))
            (:`OnCallFailed`
              (`KismetSystemLibrary.PrintString` "Unable to find session indicated by session follow request." :!label _label_2))
            (:`OnSingleSessionResultComplete`
              (if (not _bwassuccessful)
                (goto _label_2)))))))))

(fn `Can Kick Member`
  (params (`Party Id` :type "/Game/ExampleOSS/Common/BaseTasks/Parties/BasePartyIdReference Object Reference") (`Party Member Id` :type "/Game/ExampleOSS/Common/BaseTasks/Parties/BasePartyMemberIdReference Object Reference"))
  (returns (Allowed :type Boolean))
  ;[0 0 0] Only party leaders can kick members.
  (bind _is_leader_ (`self.Is Party Leader` `Party Id`))
  (if _is_leader_
    (return (not (== (`BlueprintPartyMember.GetUserId` (`/Game/ExampleOSS/Blueprints/Parties/BpPartyMemberIdReference.Party Member` (cast `/Game/ExampleOSS/Blueprints/Parties/BpPartyMemberIdReference` `Party Member Id` :!pure true))) (`OnlineHelpers.GetControllerUniqueNetId` (`GameplayStatics.GetPlayerController` 0)))))
    (else
      (return false))))

(fn `Get Invites`
  (returns (Invites :type "Array of /Game/ExampleOSS/Common/BaseTasks/Parties/BasePartyInviteReference Object Reference"))
  (locals (Results :type "Array of /Game/ExampleOSS/Common/BaseTasks/Parties/BasePartyInviteReference Object Reference"))
  (for _array_element (`OnlinePartySubsystem.GetPendingInvites` (subsystem `OnlinePartySubsystem`) (`OnlineHelpers.GetControllerUniqueNetId` (`GameplayStatics.GetPlayerController` 0)))
    (bind _returnvalue (`|GenericCreateObject` (`GameplayStatics.GetPlayerController` 0) "/Game/ExampleOSS/Blueprints/Parties/BpPartyInviteReference.BpPartyInviteReference_C" _array_element))
    (`KismetArrayLibrary.Array_Add` (`local.Results`) _returnvalue))
  (return (`local.Results`)))

(fn `Get Joined Parties`
  (returns (Parties :type "Array of /Game/ExampleOSS/Common/BaseTasks/Parties/BasePartyIdReference Object Reference"))
  (locals (Results :type "Array of /Game/ExampleOSS/Common/BaseTasks/Parties/BasePartyIdReference Object Reference"))
  (for _array_element (`OnlinePartySubsystem.GetJoinedParties` (subsystem `OnlinePartySubsystem`) (`OnlineHelpers.GetControllerUniqueNetId` (`GameplayStatics.GetPlayerController` 0)))
    (bind _returnvalue (`|GenericCreateObject` (`GameplayStatics.GetPlayerController` 0) "/Game/ExampleOSS/Blueprints/Parties/BpPartyIdReference.BpPartyIdReference_C" _array_element))
    (`KismetArrayLibrary.Array_Add` (`local.Results`) _returnvalue))
  (return (`local.Results`)))

(fn `Get Party Members`
  (params (`Party Id` :type "/Game/ExampleOSS/Common/BaseTasks/Parties/BasePartyIdReference Object Reference"))
  (returns (`Party Member Ids` :type "Array of /Game/ExampleOSS/Common/BaseTasks/Parties/BasePartyMemberIdReference Object Reference"))
  (locals (Results :type "Array of /Game/ExampleOSS/Common/BaseTasks/Parties/BasePartyMemberIdReference Object Reference"))
  (for _array_element (`OnlinePartySubsystem.GetPartyMembers` (subsystem `OnlinePartySubsystem`) (`OnlineHelpers.GetControllerUniqueNetId` (`GameplayStatics.GetPlayerController` 0)) (`/Game/ExampleOSS/Blueprints/Parties/BpPartyIdReference.Party Id` (cast `/Game/ExampleOSS/Blueprints/Parties/BpPartyIdReference` `Party Id` :!pure true)))
    (bind _returnvalue (`|GenericCreateObject` (`GameplayStatics.GetPlayerController` 0) "/Game/ExampleOSS/Blueprints/Parties/BpPartyMemberIdReference.BpPartyMemberIdReference_C" _array_element))
    (`KismetArrayLibrary.Array_Add` (`local.Results`) _returnvalue))
  (return (`local.Results`)))

(fn `Is Party Leader`
  (params (`Party Id` :type "/Game/ExampleOSS/Common/BaseTasks/Parties/BasePartyIdReference Object Reference"))
  (returns (`Is Leader?` :type Boolean))
  (bind _returnvalue (`OnlineHelpers.GetControllerUniqueNetId` (`GameplayStatics.GetPlayerController` 0)))
  (return (`OnlinePartySubsystem.IsMemberLeader` (subsystem `OnlinePartySubsystem`) _returnvalue (`/Game/ExampleOSS/Blueprints/Parties/BpPartyIdReference.Party Id` (cast `/Game/ExampleOSS/Blueprints/Parties/BpPartyIdReference` `Party Id` :!pure true)) _returnvalue)))

(fn `UserConstructionScript`
  (`parent.UserConstructionScript`))