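; Task actor from the ExampleOSS user cloud example that lists the files in the first player's cloud storage.
; It runs the async EnumerateUserFiles call on the Online User Cloud subsystem, then fetches the file list and wraps each entry in a BpFileEntry object.
; It broadcasts OnComplete with a success flag and those entries, or an empty list on failure, then destroys itself.
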(event `self.Enumerate User Files`
  (bind _returnvalue (subsystem `OnlineUserCloudSubsystem`))
  (bind (_bwassuccessful _userid) (`OnlineUserCloudSubsystemEnumerateUserFiles.EnumerateUserFiles` _returnvalue (`OnlineHelpers.GetControllerUniqueNetId` (`GameplayStatics.GetPlayerController` 0)))
    (:`OnCallFailed`
      (`self.On Complete` false (`|MakeArray`) :!label _label)
      (`self.K2_DestroyActor`))
    (:`OnEnumerateUserFilesComplete`
      (if _bwassuccessful
        (bind _userfiles (`OnlineUserCloudSubsystem.GetUserFileList` _returnvalue _userid))
        (set `self.Files` (`|MakeArray`))
        (for _array_element _userfiles
          (bind _returnvalue_2 (`|GenericCreateObject` "/Game/ExampleOSS/Blueprints/UserCloud/BpFileEntry.BpFileEntry_C" self _array_element))
          (`KismetArrayLibrary.Array_Add` (`self.Files`) _returnvalue_2))
        (`self.On Complete` true (`self.Files`))
        (`self.K2_DestroyActor`)
        (else
          (goto _label))))))

(fn `UserConstructionScript`
  (`parent.UserConstructionScript`))