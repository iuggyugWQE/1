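; Short-lived task actor in the ExampleOSS Ecom example that starts an online store checkout for a map of offers and quantities.
; PurchaseOffer logs each entry and turns those with positive quantity into purchase offers.
; It sends them through an async OnlinePurchaseSubsystem Checkout for player controller 0's net ID.
; It reports success or failure through OnPurchaseStarted, printing the error on failure, then destroys itself.
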(event `self.Purchase Offer`
  (params (`Offers to Purchase` :type "Map of String to Integer"))
  (set `self.Purchase Offers` (`|MakeArray`))
  (bind _keys (`BlueprintMapLibrary.Map_Keys` `Offers to Purchase`))
  (for _array_element _keys
    (bind _value (`BlueprintMapLibrary.Map_Find` `Offers to Purchase` _array_element))
    (`KismetSystemLibrary.PrintString` (`KismetStringLibrary.Concat_StrStr` _array_element " = " (`KismetStringLibrary.Conv_IntToString` _value) " (purchasing)"))
    (if (> _value 0)
      (`KismetArrayLibrary.Array_Add` (`self.Purchase Offers`) (make `PurchaseOfferEntryBP` "" _array_element _value))))
  (bind _result (`OnlinePurchaseSubsystemCheckout.Checkout` (subsystem `OnlinePurchaseSubsystem`) (`OnlineHelpers.GetControllerUniqueNetId` (`GameplayStatics.GetPlayerController` 0)) (make `PurchaseCheckoutRequestBP` "" (`self.Purchase Offers`)))
    (:`OnCallFailed`
      (`KismetSystemLibrary.PrintString` (`KismetTextLibrary.Conv_TextToString` (`.ErrorMessage` (break `OnlineErrorInfo` _result))) :!label _label)
      (`self.On Purchase Started` false)
      (`self.K2_DestroyActor`))
    (:`OnPurchaseCheckoutComplete`
      (if (break `OnlineErrorInfo` _result)
        (`self.On Purchase Started` true)
        (`self.K2_DestroyActor`)
        (else
          (goto _label))))))

(fn `UserConstructionScript`
  (`parent.UserConstructionScript`))