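; BpEntitlementReference wraps an Entitlement for the ecommerce part of the ExampleOSS online subsystem example.
; Four getters forward to the wrapped object and expose its ID, title, status and quantity.
; The title is the entitlement name converted to Text, and the quantity is its remaining count.
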(fn `Get Id`
  (returns (Id :type String))
  (return (`OnlineEntitlement.GetId` (`self.Entitlement`))))

(fn `Get Quantity`
  (returns (Quantity :type Integer))
  (return (`OnlineEntitlement.GetRemainingCount` (`self.Entitlement`))))

(fn `Get Status`
  (returns (Status :type String))
  (return (`OnlineEntitlement.GetStatus` (`self.Entitlement`))))

(fn `Get Title`
  (returns (Title :type Text))
  (return (`KismetTextLibrary.Conv_StringToText` (`OnlineEntitlement.GetName` (`self.Entitlement`)))))