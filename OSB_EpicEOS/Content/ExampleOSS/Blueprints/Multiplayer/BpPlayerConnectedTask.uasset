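; Server-side task for the online subsystem example that handles a player connecting to a multiplayer session.
; It caches the player's unique net ID on MultiplayerPlayerState for unregistering at logout, then registers them with the local named session.
; Whether or not registration succeeds, a dedicated server then requests EOS voice channel credentials, using the session ID as channel name.
; Successful credentials are passed to that player's MultiplayerPlayerController; failures only print messages.
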(event `self.On Player Connected`
  (params (`Player Controller` :type "PlayerController Object Reference"))
  ;[0 0 0] When a player disconnects, their unique net ID has already been removed from their PlayerController, so we won't be able to use "Get Controller Unique Net Id" during OnLogout. Store it separately in the player state here so we can use that to unregister the player properly.
  (bind _output_get (set `/Game/ExampleOSS/Common/Multiplayer/MultiplayerPlayerState.Unique Net Id` (`OnlineHelpers.GetControllerUniqueNetId` `Player Controller`) (cast `/Game/ExampleOSS/Common/Multiplayer/MultiplayerPlayerState` (`Controller.PlayerState` `Player Controller`) :!pure true)))
  (bind _array (`|MakeArray` _output_get))
  (bind (_sessionname _playerids _bwassuccessful) (`OnlineSessionSubsystemRegisterPlayers.RegisterPlayers` (subsystem `OnlineSessionSubsystem`) "MyLocalSessionName" _array)
    (:`OnCallFailed`
      (`KismetSystemLibrary.PrintString` "Failed to register player." :!label _label))
    (:`OnRegisterPlayersComplete`
      (if _bwassuccessful
        _
        (else
          (goto _label)))))
  (if (`KismetSystemLibrary.IsDedicatedServer`)
    (`KismetSystemLibrary.PrintString` "Attempting to issue voice RTC token")
    (bind _returnvalue (`OnlineSessionSubsystem.GetNamedSession` (subsystem `OnlineSessionSubsystem`) "MyLocalSessionName"))
    (bind _returnvalue_2 (`OnlineIdentitySubsystem.CreateUniquePlayerId` (subsystem `OnlineIdentitySubsystem`) "DEDICATED_SERVER"))
    (bind (_returnvalue_sessionname _returnvalue_bhosting _returnvalue_localownerid _returnvalue_registeredplayers _returnvalue_sessionstate _returnvalue_owninguserid _returnvalue_owningusername _returnvalue_sessionsettings _returnvalue_sessioninfo _returnvalue_numopenprivateconnections _returnvalue_numopenpublicconnections _returnvalue_sessionid) (break `NamedOnlineSessionBP` (`NamedOnlineSession.GetValue` _returnvalue)))
    ;[0 0 0] You can use any value for Channel Name in EOS, but we use the session ID to easily get something unique.
    (bind (_result _localuserid _credentials) (`OnlineVoiceAdminSubsystemCreateChannelCredentials.CreateChannelCredentials` (subsystem `OnlineVoiceAdminSubsystem`) _returnvalue_2 _returnvalue_sessionid _array)
      (:`OnVoiceAdminCreateChannelCredentialsComplete`
        (if (break `OnlineErrorInfo` _result)
          (bind _asmultiplayer_player_controller (cast `/Game/ExampleOSS/Common/Multiplayer/MultiplayerPlayerController` `Player Controller`))
          (bind (_output_targetuserid _output_playername _output_channelcredentials) (break `VoiceAdminChannelCredentialsBP` (`|GetArrayItem` _credentials)))
          (`/Game/ExampleOSS/Common/Multiplayer/MultiplayerPlayerController.Receive Voice Channel Credentials` _asmultiplayer_player_controller _returnvalue_sessionid _output_channelcredentials)
          (else
            (`KismetSystemLibrary.PrintString` "Failed to issue voice RTC token")))))))

(fn `UserConstructionScript`
  (`parent.UserConstructionScript`))