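; BpCreateLobbyTask is a one-shot task actor that creates an online lobby for the first local player through OnlineLobbySubsystem.
; CreateLobby builds a public, capacity-limited transaction with type, voice chat, bucket and test-integer metadata, then runs the async lobby call.
; On success it wraps the lobby in a BpLobbyRef and adds it to BpLobbyServices' JoinedLobbies.
; Either outcome is reported through CallOnComplete before the actor destroys itself.
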(event `self.Create Lobby`
  (params (`Test Attribute Value` :type Integer64) (`Lobby Services` :type "/Game/ExampleOSS/Common/BaseTasks/Lobbies/BaseLobbyServices Object Reference"))
  (bind _returnvalue (subsystem `OnlineLobbySubsystem`))
  (bind _returnvalue_2 (`OnlineLobbySubsystem.MakeCreateLobbyTransaction` _returnvalue (`OnlineHelpers.GetControllerUniqueNetId` (`GameplayStatics.GetPlayerController` 0))))
  (`OnlineLobbyTransaction.SetPublic` _returnvalue_2 true)
  (`OnlineLobbyTransaction.SetCapacity` _returnvalue_2 4)
  (`OnlineLobbyTransaction.SetMetadataByMap` _returnvalue_2 (`|MakeMap` "Type" (make `VariantDataBP` "String" false 0 0.0 0 "Lobby") "EOSVoiceChat_Enabled" (make `VariantDataBP` "Bool" true) "TestInteger" (make `VariantDataBP` "Int64" false 0 0.0 `Test Attribute Value`) "bucket" (make `VariantDataBP` "String" false 0 0.0 0 "hello")))
  (bind (_error _userid _lobby) (`OnlineLobbySubsystemCreateLobby.CreateLobby` _returnvalue (`OnlineHelpers.GetControllerUniqueNetId` (`GameplayStatics.GetPlayerController` 0)) _returnvalue_2)
    (:`OnCallFailed`
      (`self.On Complete` false :!label _label))
    (:`OnLobbyCreateOrConnectComplete`
      (if (break `OnlineErrorInfo` _error)
        (bind _returnvalue_3 (`|GenericCreateObject` `Lobby Services` "/Game/ExampleOSS/Blueprints/Lobbies/BpLobbyRef.BpLobbyRef_C" _lobby))
        (`KismetArrayLibrary.Array_Add` (`/Game/ExampleOSS/Blueprints/Lobbies/BpLobbyServices.Joined Lobbies` (cast `/Game/ExampleOSS/Blueprints/Lobbies/BpLobbyServices` `Lobby Services` :!pure true)) _returnvalue_3)
        (`self.On Complete` true _returnvalue_3)
        (else
          (goto _label)))))
  (`self.K2_DestroyActor`))

(fn `UserConstructionScript`
  (`parent.UserConstructionScript`))