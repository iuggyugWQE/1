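; Wrapper around an online subsystem friend in the OSS example, exposing identity, invite and presence data as display-ready values.
; Getters convert user IDs, names, status enums, last-online time and presence properties to strings, alongside boolean presence flags.
; Invite status decides accept, reject and delete permissions, with deletion also requiring a "deletable" attribute.
; Additional information reads eosSynthetic attributes to list each linked subsystem's ID and names.
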(fn `Can Accept Invite`
  (returns (Result :type Boolean))
  (return (select `EInviteStatus_` (`OnlineFriendRef.GetInviteStatus` (`self.Friend`)) :`PendingInbound` true)))

(fn `Can Delete Friend`
  (returns (Result :type Boolean))
  (bind _friend (`self.Friend`))
  (bind (_found _returnvalue) (`OnlineUserRef.GetUserAttribute` _friend "deletable"))
  (return (and (select `EInviteStatus_` (`OnlineFriendRef.GetInviteStatus` _friend) :`Accepted` true :`PendingOutbound` true) _found (`KismetStringLibrary.EqualEqual_StrStr` _returnvalue "true"))))

(fn `Can Reject Invite`
  (returns (Result :type Boolean))
  (return (select `EInviteStatus_` (`OnlineFriendRef.GetInviteStatus` (`self.Friend`)) :`PendingInbound` true)))

(fn `Get Additional Information`
  (returns (Value :type String))
  (locals (WrapperText :type "Array of String"))
  (bind _friend (`self.Friend`))
  (bind (_found _returnvalue) (`OnlineUserRef.GetUserAttribute` (`self.Friend`) "eosSynthetic.subsystemNames"))
  (if _found
    (for _array_element (`KismetStringLibrary.ParseIntoArray` _returnvalue ",")
      (`KismetArrayLibrary.Array_Add` (`local.WrapperText`) (`KismetStringLibrary.Concat_StrStr` "subsystem: " _array_element " id: " (`.ReturnValue` (`OnlineUserRef.GetUserAttribute` _friend (`KismetStringLibrary.Concat_StrStr` "eosSynthetic.friend." _array_element ".id"))) " real name: " (`.ReturnValue` (`OnlineUserRef.GetUserAttribute` _friend (`KismetStringLibrary.Concat_StrStr` "eosSynthetic.friend." _array_element ".realName"))) " display name: " (`.ReturnValue` (`OnlineUserRef.GetUserAttribute` _friend (`KismetStringLibrary.Concat_StrStr` "eosSynthetic.friend." _array_element ".displayName"))))))
    (return (`KismetStringLibrary.JoinStringArray` (`local.WrapperText`) " \n"))
    (else
      (return ""))))

(fn `Get Display Name`
  (returns (Value :type String))
  (return (`OnlineUserRef.GetDisplayName` (`self.Friend`))))

(fn `Get Invite Status`
  (returns (Status :type String))
  (return (`|GetEnumeratorNameAsString` (`OnlineFriendRef.GetInviteStatus` (`self.Friend`)))))

(fn `Get Presence Last Online`
  (returns (Result :type String))
  (return (`KismetTextLibrary.Conv_TextToString` (`KismetTextLibrary.AsTimeZoneDateTime_DateTime` (`.LastOnline` (break `OnlineUserPresenceData` (`OnlineFriendRef.GetPresence` (`self.Friend`))))))))

(fn `Get Presence Session ID`
  (returns (State :type String))
  (return (`OnlineHelpers.Conv_FUniqueNetIdReplToString` (break `OnlineUserPresenceData` (`OnlineFriendRef.GetPresence` (`self.Friend`))))))

(fn `Get Presence Status Properties`
  (returns (Result :type String))
  (locals (Entries :type "Array of String"))
  (bind _returnvalue (`OnlineFriendRef.GetPresence` (`self.Friend`)))
  (bind _keys (`BlueprintMapLibrary.Map_Keys` (`.Properties` (break `OnlineUserPresenceStatusData` (`.Status` (break `OnlineUserPresenceData` _returnvalue))))))
  (for _array_element _keys
    (`KismetArrayLibrary.Array_Add` (`local.Entries`) (`KismetStringLibrary.Concat_StrStr` _array_element "=" (`BlueprintMapLibrary.Map_Find` (`.Properties` (break `OnlineUserPresenceStatusData` (`.Status` (break `OnlineUserPresenceData` _returnvalue)))) _array_element))))
  (return (`KismetStringLibrary.JoinStringArray` (`local.Entries`) " \n")))

(fn `Get Presence Status State`
  (returns (State :type String))
  (return (`|GetEnumeratorNameAsString` (`.State` (break `OnlineUserPresenceStatusData` (`.Status` (break `OnlineUserPresenceData` (`OnlineFriendRef.GetPresence` (`self.Friend`)))))))))

(fn `Get Presence Status String`
  (returns (Result :type String))
  (return (break `OnlineUserPresenceStatusData` (`.Status` (break `OnlineUserPresenceData` (`OnlineFriendRef.GetPresence` (`self.Friend`)))))))

(fn `Get Real Name`
  (returns (Value :type String))
  (return (`OnlineUserRef.GetRealName` (`self.Friend`))))

(fn `Get User ID String`
  (returns (Value :type String))
  (return (`OnlineHelpers.Conv_FUniqueNetIdReplToString` (`OnlineUserRef.GetUserId` (`self.Friend`)))))

(fn `Get User ID Type`
  (returns (Value :type String))
  (return (`KismetStringLibrary.Conv_NameToString` (`OnlineHelpers.FUniqueNetIdGetType` (`OnlineUserRef.GetUserId` (`self.Friend`))))))

(fn `Has Voice Support?`
  (returns (Result :type Boolean))
  (return (`.HasVoiceSupport` (break `OnlineUserPresenceData` (`OnlineFriendRef.GetPresence` (`self.Friend`))))))

(fn `Is Joinable?`
  (returns (Result :type Boolean))
  (return (`.IsJoinable` (break `OnlineUserPresenceData` (`OnlineFriendRef.GetPresence` (`self.Friend`))))))

(fn `Is Presence Online?`
  (returns (Result :type Boolean))
  (return (`.IsOnline` (break `OnlineUserPresenceData` (`OnlineFriendRef.GetPresence` (`self.Friend`))))))

(fn `Is Presence Playing this Game?`
  (returns (Result :type Boolean))
  (return (`.IsPlayingThisGame` (break `OnlineUserPresenceData` (`OnlineFriendRef.GetPresence` (`self.Friend`))))))

(fn `Is Presence Playing?`
  (returns (Result :type Boolean))
  (return (`.IsPlaying` (break `OnlineUserPresenceData` (`OnlineFriendRef.GetPresence` (`self.Friend`))))))